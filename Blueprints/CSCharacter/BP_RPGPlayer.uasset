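; First-person RPG player character that links inventory, quests and their UI.
; GiveItem picks up ammo and caps added amounts by MaxWeight using DT_ItemInfo weights, while Y runs the first stored item's action object.
; Quests are instantiated at runtime with requirements, which helper functions mark fulfilled for named actions or conversations.
; Inventory and container widgets switch input mode and cursor, and crouching adjusts camera height.
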(event Custom|ForceCloseInventory_Event
  (bind (_player _success) (Utilities|GetPlayerController))
  (Widget|SetVisibility (Variables|Default|GetInventoryHUD) "Hidden")
  (if _success
    (Input|SetInputModeGameOnly _player)
    (Variables|/Script/Engine.PlayerController|SetbShowMouseCursor _player false)))

(event EventBeginPlay
  (|CallParentFunction)
  (bind _returnvalue (UserInterface|CreateWidget "/Game/Blueprints/UI/Management/InventoryDisplay/UMG_PlayerInventoryDisplay.UMG_PlayerInventoryDisplay_C" 0 self true))
  (UserInterface|Viewport|AddtoViewport _returnvalue 0)
  (bind _output_get (Variables|Default|SetInventoryHUD _returnvalue))
  (Widget|SetVisibility _output_get "Hidden"))

(event Collision|EventActorBeginOverlap
  (params (OtherActor :type Actor%20Object%20Reference)))

(event EventUpdateMeshPositiononCrouch
  (params (isCrouching :type Boolean))
  (bind _firstpersoncameracomponent (Variables|Default|GetFirstPersonCameraComponent))
  (bind _relativelocation (Variables|/Script/Engine.SceneComponent|GetRelativeLocation _firstpersoncameracomponent))
  (bind (_x _y) (Math|Vector|BreakVector _relativelocation))
  (Transformation|SetRelativeLocation _firstpersoncameracomponent (Math|Vector|MakeVector _x _y (select isCrouching 4e+01 8e+01)) false false))

(event EventForceCompleteQuest
  (params (Quest :type Quest%20Base%20Class%20Reference))
  (bind _returnvalue (Class|QuestSystemComponent|FinishQuest (Variables|Default|GetQuestSystem)))
  (if _returnvalue
    (Development|PrintString "Hello")
    (Audio|PlaySound2D "/Game/Music/Quest/mus_success.mus_success" 1.0 1.0 0.0 0 0)))

(event EventGiveQuest
  (params (Quest :type Quest%20Base%20Class%20Reference) (Requirements :type Array%20of%20Quest%20Requirement%20Base%20Object%20References))
  (bind _returnvalue (Game|ConstructObjectfromClass Quest self))
  (Variables|/Script/PropHunt.QuestBase|SetRequirementes _returnvalue Requirements)
  (Variables|/Script/PropHunt.QuestSystemComponent|SetCurrentQuest (Variables|Default|GetQuestSystem) _returnvalue)
  (Development|PrintString "Given"))

(event Input|ActionEvents|InputActionManagmentDisplayInventory
  (params (Key :type Key%20Structure :default "None"))
  (bind (_player _success) (Utilities|GetPlayerController))
  (bind _inventoryhud (Variables|Default|GetInventoryHUD))
  (:Pressed
    (if (Widget|IsVisible _inventoryhud)
      (Widget|SetVisibility _inventoryhud "Hidden")
      (if _success
        (Input|SetInputModeGameOnly _player)
        (Variables|/Script/Engine.PlayerController|SetbShowMouseCursor _player false))
      (else
        (Default|Update _inventoryhud)
        (Widget|SetVisibility _inventoryhud "Visible")
        (if _success
          (Input|SetInputModeUIOnly _player _inventoryhud "DoNotLock")
          (Variables|/Script/Engine.PlayerController|SetbShowMouseCursor _player true)
          (Default|OnDisplayedEvent _inventoryhud))))))

(event Input|KeyboardEvents|Y
  (params (Key :type Key%20Structure :default "None"))
  (bind _inventory (Variables|Default|GetInventory))
  (bind _storeditems (Variables|/Script/PropHunt.InventoryComponent|GetStoredItems _inventory))
  (bind _output (Utilities|Array|Get(acopy) _storeditems))
  (bind (_name _amount _description _biskey _keyid _itemaction) (Utilities|Struct|BreakBuildingItemInfo _output))
  (:Pressed
    (if (> (Utilities|Array|Length _storeditems) 0)
      (bind _returnvalue (Game|ConstructObjectfromClass _itemaction self))
      (Class|ItemActionObjectBase|PerformAction _returnvalue self _name))))

(fn ConstructionScript
  (|CallParentFunction))

(fn CalculateTotalWieghtOfInventory
  (for _array_element (Variables|/Script/PropHunt.InventoryComponent|GetStoredItems (Variables|Default|GetInventory))
    (bind _returnvalue (Utilities|GetDataTableRow "/Game/DataTable/Managment/DT_ItemInfo.DT_ItemInfo" (Utilities|String|StringToName (.Name (Utilities|Struct|BreakBuildingItemInfo _array_element))))
      (:then
        (LocalVariables|SetTemp (+ (* (.Amount (Utilities|Struct|BreakBuildingItemInfo _array_element)) (.Weight (Utilities|Struct|BreakS_ItemDescription _returnvalue))) (LocalVariables|GetTemp))))))
  (return (LocalVariables|GetTemp)))

(fn HasKeywithId
  (params (id :type Integer))
  (return (Class|InventoryComponent|HasKey (Variables|Default|GetInventory) id)))

(fn CompleteQuestPerformAction
  (params (Name :type Name :default "None"))
  (for _array_element (Variables|/Script/PropHunt.QuestBase|GetRequirementes (Variables|/Script/PropHunt.QuestSystemComponent|GetCurrentQuest (Variables|Default|GetQuestSystem)))
    (if (Utilities|Name|Equal(Name) (Variables|/Script/PropHunt.QuestRequirementBase|GetName _array_element) Name)
      (Variables|/Script/PropHunt.QuestRequirementBase|SetbFulfilled _array_element true)
      (return true)))
  (return false))

(fn CompleteQuestTalktoSomeone
  (params (Someone :type Actor%20Object%20Reference))
  (for _array_element (Variables|/Script/PropHunt.QuestBase|GetRequirementes (Variables|/Script/PropHunt.QuestSystemComponent|GetCurrentQuest (Variables|Default|GetQuestSystem)))
    (bind _asqr_talk_to_someone (Utilities|Casting|CastToQR_TalkToSomeone _array_element))
    (if (== Someone (Variables|/Game/Blueprints/QuestSystem/QuestRequirements/QR_TalkToSomeone.QR_TalkToSomeone_C|GetWhoToTalkTo _asqr_talk_to_someone))
      (Variables|/Script/PropHunt.QuestRequirementBase|SetbFulfilled _asqr_talk_to_someone true)
      (return (== Someone (Variables|/Game/Blueprints/QuestSystem/QuestRequirements/QR_TalkToSomeone.QR_TalkToSomeone_C|GetWhoToTalkTo _asqr_talk_to_someone)))))
  (return false))

(fn GiveItem
  (params (item :type Building%20Item%20Info%20Structure))
  (bind (_name _amount _description _biskey _keyid _itemaction _ammo) (Utilities|Struct|BreakBuildingItemInfo item))
  (bind _total (CallFunction|CalculateTotalWieghtOfInventory))
  (bind _inventory (Variables|Default|GetInventory))
  (CallFunction|PickUpAmmo _ammo)
  ;[1 1 1] Calculate Items
  (if (== _amount 0)
    (return 0 false)
    (else
      (bind _returnvalue (Utilities|GetDataTableRow "/Game/DataTable/Managment/DT_ItemInfo.DT_ItemInfo" (Utilities|String|StringToName _name))
        (:then
          (if (== _total 0.0)
            (Class|InventoryComponent|AddItem _inventory (Utilities|Struct|MakeBuildingItemInfo _name (select (== (.Weight (Utilities|Struct|BreakS_ItemDescription _returnvalue)) 0.0) _amount (select (>= (Math|Float|Truncate (/ (Variables|Default|GetMaxWeight) (.Weight (Utilities|Struct|BreakS_ItemDescription _returnvalue)))) _amount) _amount (Math|Float|Truncate (/ (Variables|Default|GetMaxWeight) (.Weight (Utilities|Struct|BreakS_ItemDescription _returnvalue)))))) _description _biskey _keyid _itemaction _ammo))
            (bind _output_get (LocalVariables|SetTempValue (select (== (.Weight (Utilities|Struct|BreakS_ItemDescription _returnvalue)) 0.0) _amount (select (>= (Math|Float|Truncate (/ (Variables|Default|GetMaxWeight) (.Weight (Utilities|Struct|BreakS_ItemDescription _returnvalue)))) _amount) _amount (Math|Float|Truncate (/ (Variables|Default|GetMaxWeight) (.Weight (Utilities|Struct|BreakS_ItemDescription _returnvalue))))))))
            (return (- _amount _output_get) true)
            (elif (or (== (.Weight (Utilities|Struct|BreakS_ItemDescription _returnvalue)) 0.0) (> (Math|Float|Truncate (/ (- (Variables|Default|GetMaxWeight) _total) (.Weight (Utilities|Struct|BreakS_ItemDescription _returnvalue)))) 0))
              _
              (else
                (return 0 false)))))
        (:RowNotFound
          _))
      (bind _output_get_2 (LocalVariables|SetTempValue (select (== (.Weight (Utilities|Struct|BreakS_ItemDescription _returnvalue)) 0.0) _amount (select (>= (Math|Float|Truncate (/ (- (Variables|Default|GetMaxWeight) _total) (.Weight (Utilities|Struct|BreakS_ItemDescription _returnvalue)))) _amount) _amount (Math|Float|Truncate (/ (- (Variables|Default|GetMaxWeight) _total) (.Weight (Utilities|Struct|BreakS_ItemDescription _returnvalue))))))))
      (Class|InventoryComponent|AddItem _inventory (Utilities|Struct|MakeBuildingItemInfo _name (select (== (.Weight (Utilities|Struct|BreakS_ItemDescription _returnvalue)) 0.0) _amount (select (>= (Math|Float|Truncate (/ (- (Variables|Default|GetMaxWeight) _total) (.Weight (Utilities|Struct|BreakS_ItemDescription _returnvalue)))) _amount) _amount (Math|Float|Truncate (/ (- (Variables|Default|GetMaxWeight) _total) (.Weight (Utilities|Struct|BreakS_ItemDescription _returnvalue)))))) _description _biskey _keyid _itemaction _ammo))
      (return (- _amount _output_get_2) true))))

(fn RequestDisplayInteractionWidget
  (params (item :type Pickupable%20Item%20Object%20Reference))
  (Utilities|IsValid item
    (:Is%20Valid
      (bind _returnvalue (UserInterface|CreateWidget "/Game/Blueprints/UI/Management/ItemContainersInteractions/UMG_ContainerDisplay.UMG_ContainerDisplay_C" 0 item self))
      (bind _output_get (Variables|Default|SetItemInteractionDisplay _returnvalue))
      (UserInterface|Viewport|AddtoViewport _output_get 0)
      (bind _asplayer_controller (Utilities|Casting|CastToPlayerController (Pawn|GetController)))
      (Input|SetInputModeUIOnly _asplayer_controller _output_get "DoNotLock")
      (Variables|/Script/Engine.PlayerController|SetbShowMouseCursor _asplayer_controller true))
    (:Is%20Not%20Valid
      (return false))))

(fn RequestHideContainerDisplay
  (Default|OnRemovefromParentEvent (Variables|Default|GetItemInteractionDisplay))
  (Widget|RemovefromParent (Variables|Default|GetItemInteractionDisplay))
  (Variables|Default|SetItemInteractionDisplay 0)
  (bind _asplayer_controller (Utilities|Casting|CastToPlayerController (Pawn|GetController)))
  (Variables|/Script/Engine.PlayerController|SetbShowMouseCursor _asplayer_controller false)
  (Input|SetInputModeGameOnly _asplayer_controller)
  (return true))