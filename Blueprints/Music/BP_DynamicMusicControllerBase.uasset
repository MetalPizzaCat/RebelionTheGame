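; Base Blueprint for a dynamic music controller, supplying soldier-state queries; it has no music playback logic itself.
; CanThisSolderSeePlayer treats a soldier as seeing the player when its current target is a valid BP_CSCharacter.
; IsEveryoneDead returns true only when every entry in SoldersToCareAbout reports dead, including when the list is empty.
; Both functions override parent versions without calling them, querying soldiers through message calls, and the event graph is empty.
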(event EventBeginPlay)

(event Collision|EventActorBeginOverlap
  (params (OtherActor :type Actor%20Object%20Reference)))

(event EventTick
  (params (DeltaSeconds :type Float%20%28single-precision%29)))

(fn ConstructionScript)

(fn CanThisSolderSeePlayer
  (params (Solder :type Actor%20Object%20Reference))
  (bind _target (Class|BPIAI|GetCurrentTarget(Message) Solder))
  (Utilities|IsValid _target
    (:Is%20Valid
      (Utilities|Casting|CastToBP_CSCharacter _target
        (:then
          (return true))
        (:CastFailed
          _)))
    (:Is%20Not%20Valid
      _))
  (return false))

(fn IsEveryoneDead
  (for _array_element (Variables|Default|GetSoldersToCareAbout)
    (bind _is (Class|BPIAI|IsDead(Message) _array_element))
    (if (not _is)
      (return false)))
  (return true))