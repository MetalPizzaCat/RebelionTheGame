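; BP_Explosive is a damageable actor that catches fire when weakened and explodes when its Health runs out.
; AnyDamage subtracts Health; at half of 100 or lower it shows the fire particles, calls OnSetOnFire and starts a fast looping timer.
; That timer keeps draining Health through the same check until zero, when it plays sound and effect, applies radial falloff damage ignoring itself, and destroys itself.
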(event Custom|BeingOnFire_Event
  (bind _returnvalue (Transformation|GetActorLocation))
  (bind _damageradius (Variables|Default|GetDamageRadius))
  (bind _basedamage (Variables|Default|GetBaseDamage))
  (Variables|Default|SetHealth (- (Variables|Default|GetHealth) 0.1))
  (if (<= (stale Game|Damage|EventAnyDamage _output_get) 0.0)
    (Audio|PlaySoundatLocation (Variables|Default|GetExplosionSound) _returnvalue "0, 0, 0" 1.0 1.0 0.0 "/Game/SuperGrid/TutorialLevel/SoundEffects/Attenuation_Ambient.Attenuation_Ambient" 0 0)
    (Effects|SpawnEmitteratLocation (Variables|Default|GetExplosionEffect) _returnvalue)
    (bind _returnvalue_2 (Class|GameplayStatics|ApplyRadialDamagewithFalloff _basedamage (* _basedamage 0.2) _returnvalue _damageradius (+ _damageradius (/ _damageradius 5.0)) 1.0 "/Script/Engine.DamageType" (Utilities|Array|MakeArray self) 0 0 "ECC_Visibility"))
    (Actor|DestroyActor)
    (elif (<= (stale Game|Damage|EventAnyDamage _output_get) 5e+01)
      (if (not (Utilities|Time|IsValidTimerHandle (Variables|Default|GetOnFireDamageTimer)))
        (Rendering|SetVisibility (Variables|Default|GetParticleSystem) true false)
        (Default|CallOnSetonFire)
        (Variables|Default|SetOnFire true)
        (bind _returnvalue_3 (Utilities|Time|SetTimerbyEvent (delegate Custom|BeingOnFire_Event) 0.01 true))
        (Variables|Default|SetOnFireDamageTimer _returnvalue_3)))))

(event EventBeginPlay)

(event Collision|EventActorBeginOverlap
  (params (OtherActor :type Actor%20Object%20Reference)))

(event EventTick
  (params (DeltaSeconds :type Float%20%28single-precision%29)))

(event Game|Damage|EventAnyDamage
  (params (Damage :type Float%20%28single-precision%29) (DamageType :type Damage%20Type%20Object%20Reference) (InstigatedBy :type Controller%20Object%20Reference) (DamageCauser :type Actor%20Object%20Reference))
  (bind _returnvalue (Transformation|GetActorLocation))
  (bind _damageradius (Variables|Default|GetDamageRadius))
  (bind _basedamage (Variables|Default|GetBaseDamage))
  (if (> (Variables|Default|GetHealth) 0.0)
    (bind _output_get (Variables|Default|SetHealth (- (Variables|Default|GetHealth) Damage)))
    (if (<= _output_get 0.0)
      (Audio|PlaySoundatLocation (Variables|Default|GetExplosionSound) _returnvalue "0, 0, 0" 1.0 1.0 0.0 "/Game/SuperGrid/TutorialLevel/SoundEffects/Attenuation_Ambient.Attenuation_Ambient" 0 0)
      (Effects|SpawnEmitteratLocation (Variables|Default|GetExplosionEffect) _returnvalue)
      (bind _returnvalue_2 (Class|GameplayStatics|ApplyRadialDamagewithFalloff _basedamage (* _basedamage 0.2) _returnvalue _damageradius (+ _damageradius (/ _damageradius 5.0)) 1.0 "/Script/Engine.DamageType" (Utilities|Array|MakeArray self) 0 0 "ECC_Visibility"))
      (Actor|DestroyActor)
      (elif (<= _output_get 5e+01)
        (if (not (Utilities|Time|IsValidTimerHandle (Variables|Default|GetOnFireDamageTimer)))
          (Rendering|SetVisibility (Variables|Default|GetParticleSystem) true false)
          (Default|CallOnSetonFire)
          (Variables|Default|SetOnFire true)
          (bind _returnvalue_3 (Utilities|Time|SetTimerbyEvent (delegate Custom|BeingOnFire_Event) 0.01 true))
          (Variables|Default|SetOnFireDamageTimer _returnvalue_3))))))

(fn ConstructionScript)