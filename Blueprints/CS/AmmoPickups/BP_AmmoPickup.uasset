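; Ammo pickup actor that gives bullets and grenades to a player character on touch.
; A box overlap casts to BP_CSCharacter, passes its Ammo and Grenades amounts through PickUpAmmoMessage, then destroys the pickup.
; On destruction it adds its display name to the DestroyedActorManager's Actors list, if that manager is valid.
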(event OnComponentBeginOverlap(Box)
  (params (OverlappedComponent :type Primitive%20Component%20Object%20Reference) (OtherActor :type Actor%20Object%20Reference) (OtherComp :type Primitive%20Component%20Object%20Reference) (OtherBodyIndex :type Integer) (bFromSweep :type Boolean) (SweepResult :type Hit%20Result%20Structure%20%28by%20ref%29))
  (bind _asbp_cscharacter (Utilities|Casting|CastToBP_CSCharacter OtherActor))
  (Class|BPICSInteractions|PickUpAmmo(Message) _asbp_cscharacter (Variables|Default|GetAmmo) (Variables|Default|GetGrenades))
  (Actor|DestroyActor))

(event EventBeginPlay)

(event Collision|EventActorBeginOverlap
  (params (OtherActor :type Actor%20Object%20Reference)))

(event EventTick
  (params (DeltaSeconds :type Float%20%28single-precision%29)))

(event EventDestroyed
  (bind _destroyedactormanager (Variables|SaveSystem|GetDestroyedActorManager))
  (Utilities|IsValid _destroyedactormanager
    (:Is%20Valid
      (Utilities|Array|Add (Variables|/Game/Blueprints/SaveSystem/BP_DestroyedActorManager.BP_DestroyedActorManager_C|GetActors _destroyedactormanager) (Utilities|GetDisplayName self)))))

(fn ConstructionScript)