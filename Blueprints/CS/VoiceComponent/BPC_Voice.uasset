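; Voice component that plays a character's barks for alert, alarm, enemy lost, pain, death, selection and deselection.
; Each function looks up the row named by the VoiceData handle, then plays that event's sound at the given location if it is valid.
; Sounds use the shared ambient attenuation, except the enemy-lost line, which passes no attenuation settings.
; The event graph holds no logic.
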(event EventBeginPlay)

(event EventTick
  (params (DeltaSeconds :type Float%20%28single-precision%29)))

(fn VoiceAlert
  (params (Location :type Vector))
  (bind _voicedata (Variables|Default|GetVoiceData))
  (bind (_datatable _rowname) (Utilities|Struct|BreakDataTableRowHandle _voicedata))
  (bind _returnvalue (Utilities|GetDataTableRow _datatable _rowname)
    (:then
      (Utilities|IsValid (.Alert (Utilities|Struct|BreakS_VoiceData _returnvalue))
        (:Is%20Valid
          (Audio|PlaySoundatLocation (.Alert (Utilities|Struct|BreakS_VoiceData _returnvalue)) Location "0, 0, 0" 1.0 1.0 0.0 "/Game/SuperGrid/TutorialLevel/SoundEffects/Attenuation_Ambient.Attenuation_Ambient" 0 0))))))

(fn VoiceAlarm
  (params (Location :type Vector))
  (bind _voicedata (Variables|Default|GetVoiceData))
  (bind (_datatable _rowname) (Utilities|Struct|BreakDataTableRowHandle _voicedata))
  (bind _returnvalue (Utilities|GetDataTableRow _datatable _rowname)
    (:then
      (Utilities|IsValid (.Alarm (Utilities|Struct|BreakS_VoiceData _returnvalue))
        (:Is%20Valid
          (Audio|PlaySoundatLocation (.Alarm (Utilities|Struct|BreakS_VoiceData _returnvalue)) Location "0, 0, 0" 1.0 1.0 0.0 "/Game/SuperGrid/TutorialLevel/SoundEffects/Attenuation_Ambient.Attenuation_Ambient" 0 0))))))

(fn VoiceLost
  (params (Location :type Vector))
  (bind _voicedata (Variables|Default|GetVoiceData))
  (bind (_datatable _rowname) (Utilities|Struct|BreakDataTableRowHandle _voicedata))
  (bind _returnvalue (Utilities|GetDataTableRow _datatable _rowname)
    (:then
      (Utilities|IsValid (.EnemyLost (Utilities|Struct|BreakS_VoiceData _returnvalue))
        (:Is%20Valid
          (Audio|PlaySoundatLocation (.EnemyLost (Utilities|Struct|BreakS_VoiceData _returnvalue)) Location "0, 0, 0" 1.0 1.0 0.0 0 0 0))))))

(fn VoicePain
  (params (Location :type Vector))
  (bind _voicedata (Variables|Default|GetVoiceData))
  (bind (_datatable _rowname) (Utilities|Struct|BreakDataTableRowHandle _voicedata))
  (bind _returnvalue (Utilities|GetDataTableRow _datatable _rowname)
    (:then
      (Utilities|IsValid (.Pain (Utilities|Struct|BreakS_VoiceData _returnvalue))
        (:Is%20Valid
          (Audio|PlaySoundatLocation (.Pain (Utilities|Struct|BreakS_VoiceData _returnvalue)) Location "0, 0, 0" 1.0 1.0 0.0 "/Game/SuperGrid/TutorialLevel/SoundEffects/Attenuation_Ambient.Attenuation_Ambient" 0 0))))))

(fn VoiceDie
  (params (Location :type Vector))
  (bind _voicedata (Variables|Default|GetVoiceData))
  (bind (_datatable _rowname) (Utilities|Struct|BreakDataTableRowHandle _voicedata))
  (bind _returnvalue (Utilities|GetDataTableRow _datatable _rowname)
    (:then
      (Utilities|IsValid (.Death (Utilities|Struct|BreakS_VoiceData _returnvalue))
        (:Is%20Valid
          (Audio|PlaySoundatLocation (.Death (Utilities|Struct|BreakS_VoiceData _returnvalue)) Location "0, 0, 0" 1.0 1.0 0.0 "/Game/SuperGrid/TutorialLevel/SoundEffects/Attenuation_Ambient.Attenuation_Ambient" 0 0))))))

(fn VoiceRespondtoBeingSelected
  (params (Location :type Vector))
  (bind _voicedata (Variables|Default|GetVoiceData))
  (bind (_datatable _rowname) (Utilities|Struct|BreakDataTableRowHandle _voicedata))
  (bind _returnvalue (Utilities|GetDataTableRow _datatable _rowname)
    (:then
      (Utilities|IsValid (.ResponseToBeingSelected (Utilities|Struct|BreakS_VoiceData _returnvalue))
        (:Is%20Valid
          (Audio|PlaySoundatLocation (.ResponseToBeingSelected (Utilities|Struct|BreakS_VoiceData _returnvalue)) Location "0, 0, 0" 1.0 1.0 0.0 "/Game/SuperGrid/TutorialLevel/SoundEffects/Attenuation_Ambient.Attenuation_Ambient" 0 0))))))

(fn VoiceRespondtoBeingUnSelected
  (params (Location :type Vector))
  (bind _voicedata (Variables|Default|GetVoiceData))
  (bind (_datatable _rowname) (Utilities|Struct|BreakDataTableRowHandle _voicedata))
  (bind _returnvalue (Utilities|GetDataTableRow _datatable _rowname)
    (:then
      (Utilities|IsValid (.ResponseToBeingUnSelected (Utilities|Struct|BreakS_VoiceData _returnvalue))
        (:Is%20Valid
          (Audio|PlaySoundatLocation (.ResponseToBeingUnSelected (Utilities|Struct|BreakS_VoiceData _returnvalue)) Location "0, 0, 0" 1.0 1.0 0.0 "/Game/SuperGrid/TutorialLevel/SoundEffects/Attenuation_Ambient.Attenuation_Ambient" 0 0))))))