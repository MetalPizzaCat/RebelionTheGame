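; Shooting range dummy that takes point damage and ragdolls on death.
; Each hit finds the skeletal bone closest to the impact: a head hit kills instantly, while others subtract damage from Health and play a flesh impact sound until it reaches zero.
; Die enables physics simulation on the mesh, plays a spark sound and calls OnDeath to signal the kill.
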(event EventBeginPlay)

(event Collision|EventActorBeginOverlap
  (params (OtherActor :type Actor%20Object%20Reference)))

(event EventTick
  (params (DeltaSeconds :type Float%20%28single-precision%29)))

(event Game|Damage|EventAnyDamage
  (params (Damage :type Float%20%28single-precision%29) (DamageType :type Damage%20Type%20Object%20Reference) (InstigatedBy :type Controller%20Object%20Reference) (DamageCauser :type Actor%20Object%20Reference)))

(event Game|Damage|EventPointDamage
  (params (Damage :type Float%20%28single-precision%29) (DamageType :type Damage%20Type%20Object%20Reference) (HitLocation :type Vector :default "0, 0, 0") (HitNormal :type Vector :default "0, 0, 0") (HitComponent :type Primitive%20Component%20Object%20Reference) (BoneName :type Name :default "None") (ShotFromDirection :type Vector :default "0, 0, 0") (InstigatedBy :type Controller%20Object%20Reference) (DamageCauser :type Actor%20Object%20Reference) (HitInfo :type Hit%20Result%20Structure%20%28by%20ref%29))
  (if (Utilities|Name|Equal(Name) (.ReturnValue (Class|SkinnedMeshComponent|FindClosestBoneK2 (Variables|Default|GetSkeletalMesh) HitLocation 0.0)) "head")
    (CallFunction|Die)
    (else
      (bind _output_get (Variables|Default|SetHealth (- (Variables|Default|GetHealth) Damage)))
      (if (<= _output_get 0.0)
        (CallFunction|Die)
        (else
          (Audio|PlaySoundatLocation "/Game/Sounds/hl2/physics/flesh/flesh_impact_bullet_Cue.flesh_impact_bullet_Cue" (Transformation|GetActorLocation) "0, 0, 0" 1.0 1.0 0.0 0 0 0))))))

(fn ConstructionScript)

(fn Die
  (Physics|SetSimulatePhysics (Variables|Default|GetSkeletalMesh) true)
  (Audio|PlaySoundatLocation "/Game/Sounds/hl2beta/ambient/fx/electric/spark1.spark1" (Transformation|GetActorLocation) "0, 0, 0" 1.0 1.0 0.0 0 0 0)
  (Default|CallOnDeath))