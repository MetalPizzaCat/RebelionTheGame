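; BP_Solder is an AI soldier Blueprint that varies its body mesh by loadout.
; After the parent construction script runs, soldiers with a helmet get a mesh matched to rifle, pistol or sniper rifle, keeping the current mesh for other weapons.
; Soldiers without a helmet share one body mesh regardless of weapon.
; A getter exposes the flag for ignoring noise from friendlies, and the event graph adds no logic.
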(event EventBeginPlay
  (|CallParentFunction) ; This node is disabled and will not be called.\nDrag off pins to build functionality.
)

(event Collision|EventActorBeginOverlap
  (params (OtherActor :type Actor%20Object%20Reference)))

(event EventTick
  (params (DeltaSeconds :type Float%20%28single-precision%29))
  (|CallParentFunction DeltaSeconds) ; This node is disabled and will not be called.\nDrag off pins to build functionality.
)

(fn ConstructionScript
  (bind _mesh (Variables|Character|GetMesh))
  (bind _weaponclass (Variables|Default|GetWeaponClass))
  (|CallParentFunction)
  (if (Variables|Default|GetHasHelmet)
    (if (== _weaponclass "/Game/Blueprints/Weapons/BP_Rifle.BP_Rifle_C")
      (Class|SkinnedMeshComponent|SetSkeletalMesh _mesh "/Game/Customized_Soldier/Mesh/Full_Skeleton/SK_Body_2_Updated.SK_Body_2_Updated" false)
      (elif (== _weaponclass "/Game/Blueprints/Weapons/BP_Pistol.BP_Pistol_C")
        (Class|SkinnedMeshComponent|SetSkeletalMesh _mesh "/Game/Customized_Soldier/Mesh/Full_Skeleton/SK_Body_1.SK_Body_1" false)
        (elif (== _weaponclass "/Game/Blueprints/Weapons/BP_SniperRifle.BP_SniperRifle_C")
          (Class|SkinnedMeshComponent|SetSkeletalMesh _mesh "/Game/Customized_Soldier/Mesh/Full_Skeleton/SK_Body_4.SK_Body_4" false))))
    (else
      (Class|SkinnedMeshComponent|SetSkeletalMesh _mesh "/Game/Customized_Soldier/Mesh/Full_Skeleton/SK_Body_5.SK_Body_5" false))))

(fn GetIgnoreNoiseProducedbyFriendlies
  (return (Variables|Default|GetIgnoreNoiseProducedByFriendlies)))