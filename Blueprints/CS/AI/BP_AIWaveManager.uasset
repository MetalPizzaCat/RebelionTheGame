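; BP_AIWaveManager watches a group of AI and signals when every one of them is dead.
; A looping timer started at BeginPlay, paced by UpdateFrequency, polls each entry in AIToManage with an IsDead message and ANDs the results.
; When all report dead it calls OnAllAiDie; the timer is never cleared, so the call repeats on later checks while that holds.
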(event Custom|Update_Event
  (for (_array_element _array_index) (Variables|Default|GetAIToManage)
    (if (== _array_index 0)
      (bind _is (Class|BPIAI|IsDead(Message) _array_element))
      (Variables|Default|SetDead _is)
      (else
        (bind _is_2 (Class|BPIAI|IsDead(Message) _array_element))
        (Variables|Default|SetDead (and _is_2 (Variables|Default|GetDead))))))
  (if (Variables|Default|GetDead)
    (Default|CallOnAllAiDie)))

(event EventBeginPlay
  (Utilities|Time|SetTimerbyEvent (delegate Custom|Update_Event) (Variables|Default|GetUpdateFrequency) true))

(event Collision|EventActorBeginOverlap
  (params (OtherActor :type Actor%20Object%20Reference)))

(event EventTick
  (params (DeltaSeconds :type Float%20%28single-precision%29)))

(fn ConstructionScript)