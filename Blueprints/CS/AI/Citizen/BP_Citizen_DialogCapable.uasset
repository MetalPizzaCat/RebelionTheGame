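; Citizen NPC Blueprint that opens a dialogue when a character interacts with it.
; On Interact by a BP_CSCharacter, it creates a DemoDialogueWidget from its Dialog data and adds it to the viewport.
; It then registers itself and the widget as that character's current dialog target and widget.
; AddHealth, HasKeyWithId and RemoveKey are stubs that return false.
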(event EventBeginPlay
  (|CallParentFunction) ; This node is disabled and will not be called.\nDrag off pins to build functionality.
)

(event Collision|EventActorBeginOverlap
  (params (OtherActor :type Actor%20Object%20Reference))
  (|CallParentFunction OtherActor) ; This node is disabled and will not be called.\nDrag off pins to build functionality.
)

(event EventTick
  (params (DeltaSeconds :type Float%20%28single-precision%29))
  (|CallParentFunction DeltaSeconds) ; This node is disabled and will not be called.\nDrag off pins to build functionality.
)

(event EventInteract
  (params (interactor :type Actor%20Object%20Reference) (interactedComponent :type Primitive%20Component%20Object%20Reference))
  (bind _self self)
  (bind _asbp_cscharacter (Utilities|Casting|CastToBP_CSCharacter interactor))
  (bind _returnvalue (UserInterface|CreateWidget "/DialoguePlugin/UI/DemoDialogueWidget.DemoDialogueWidget_C" (.AsPlayer%20Controller (Utilities|Casting|CastToPlayerController (Pawn|GetController _asbp_cscharacter))) (Variables|Default|GetDialog) _self))
  (UserInterface|Viewport|AddtoViewport _returnvalue 0)
  (Variables|/Game/Blueprints/CSCharacter/BP_CSCharacter.BP_CSCharacter_C|SetCurrentDialogTarget _asbp_cscharacter _self)
  (Variables|/Game/Blueprints/CSCharacter/BP_CSCharacter.BP_CSCharacter_C|SetCurrentDialogWidget _asbp_cscharacter _returnvalue))

(fn ConstructionScript
  (|CallParentFunction))

(fn AddHealth
  (params (amountOfHealth :type Float%20%28single-precision%29))
  (return false))

(fn HasKeywithId
  (params (id :type Integer))
  (return false))

(fn RemoveKey
  (params (KeyId :type Integer))
  (return false))