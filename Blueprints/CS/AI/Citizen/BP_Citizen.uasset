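; BP_Citizen is a non-combat AI character that can patrol the nodes of an AINodeManager or stay idle.
; NextNode advances the node index, wrapping only for looping patrols, and GetCurrentNode returns that node unless the citizen is idle.
; Target, enemy and other combat-related queries are stubs returning empty, false or zero.
; Die unpossesses the controller, disables capsule collision, flags the citizen dead and ragdolls the mesh.
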(event EventBeginPlay)

(event Collision|EventActorBeginOverlap
  (params (OtherActor :type Actor%20Object%20Reference)))

(event EventTick
  (params (DeltaSeconds :type Float%20%28single-precision%29)))

(event EventDie
  (bind _returnvalue (Pawn|GetController))
  (Utilities|IsValid _returnvalue
    (:Is%20Valid
      (Pawn|UnPossess _returnvalue))
    (:Is%20Not%20Valid
      _))
  (Collision|SetCollisionEnabled (Variables|Default|GetCapsuleComponent) "NoCollision")
  (Variables|Default|SetbDead true)
  (Physics|SetSimulatePhysics (Variables|Character|GetMesh) true))

(event EventNextNode
  (bind _ainodemanager (Variables|Default|GetAINodeManager))
  ;[1 1 1] Next patrol
  (Math|Integer|IncrementInt (Variables|Default|GetCurrentNodeId)
    (:%20%20
      (if (>= (Variables|Default|GetCurrentNodeId) (Utilities|Array|Length (Variables|/Script/PropHunt.AINodeManagerBase|GetNodes _ainodemanager)))
        (if (Variables|/Script/PropHunt.AINodeManagerBase|GetbLoopingPatrol _ainodemanager)
          (Variables|Default|SetCurrentNodeId 0))))))

(fn ConstructionScript)

(fn GetCurrentNode
  (bind _ainodemanager (Variables|Default|GetAINodeManager))
  (if (Variables|Default|GetIdle)
    (return 0)
    (else
      (Utilities|IsValid _ainodemanager
        (:Is%20Valid
          (return (Class|AINodeManagerBase|GetNode _ainodemanager (Variables|Default|GetCurrentNodeId))))
        (:Is%20Not%20Valid
          (return 0))))))

(fn GetCurrentTarget
  (return 0))

(fn GetEnemyClasses
  (return 0))

(fn GetIsFriendlytoPlayer
  (return false))

(fn GetIsHoldingPosition
  (return false))

(fn GetNodeManager
  (return (Variables|Default|GetAINodeManager)))

(fn GetTarget
  (return 0))

(fn GetTimetoCalmDown
  (return 0.0))

(fn HasTarget
  (return false))

(fn IsDead
  (return (Variables|Default|GetbDead)))

(fn IsIdle
  (return (Variables|Default|GetIdle)))

(fn IsTalking
  (return (Variables|Default|GetTalking)))