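; BP_HealthPickup is a health pickup that offers health to actors overlapping its Box component.
; It passes its Info to the other actor through AddHealthMessage and, only if that returns true, plays a pickup sound at its location and destroys itself.
; On destruction, it adds its display name to the Actors collection of a valid DestroyedActorManager, recording that it is gone.
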(event OnComponentBeginOverlap(Box)
  (params (OverlappedComponent :type Primitive%20Component%20Object%20Reference) (OtherActor :type Actor%20Object%20Reference) (OtherComp :type Primitive%20Component%20Object%20Reference) (OtherBodyIndex :type Integer) (bFromSweep :type Boolean) (SweepResult :type Hit%20Result%20Structure%20%28by%20ref%29))
  (bind _returnvalue (Class|InteractionInterface|AddHealth(Message) OtherActor (Variables|Default|GetInfo)))
  (if _returnvalue
    (Audio|PlaySoundatLocation "/Game/Sounds/itm/Interact/PickItem2.PickItem2" (Transformation|GetActorLocation) "0, 0, 0" 1.0 1.0 0.0 "/Game/SuperGrid/TutorialLevel/SoundEffects/Attenuation_Ambient.Attenuation_Ambient" 0 0)
    (Actor|DestroyActor)))

(event EventBeginPlay)

(event Collision|EventActorBeginOverlap
  (params (OtherActor :type Actor%20Object%20Reference)))

(event EventTick
  (params (DeltaSeconds :type Float%20%28single-precision%29)))

(event EventDestroyed
  (bind _destroyedactormanager (Variables|SaveSystem|GetDestroyedActorManager))
  (Utilities|IsValid _destroyedactormanager
    (:Is%20Valid
      (Utilities|Array|Add (Variables|/Game/Blueprints/SaveSystem/BP_DestroyedActorManager.BP_DestroyedActorManager_C|GetActors _destroyedactormanager) (Utilities|GetDisplayName self)))))

(fn ConstructionScript)