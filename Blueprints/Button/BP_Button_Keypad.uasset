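; Keypad button actor that opens a code-entry widget when interacted with.
; Interact creates UMG_KeyPad, passing the required code and a self reference, then adds it to the viewport and stores it.
; The widget's success and failure events, and matching input events on the actor, each play their own 2D sound, then remove the widget and clear the reference.
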(event OnFailed(ButtonHud)
  (Audio|PlaySound2D "/Game/Retro_8Bit_Sounds/Retro_Orginal/Cues/retro_fail_sound_04_Cue.retro_fail_sound_04_Cue" 1.0 1.0 0.0 0 0)
  (Widget|RemovefromParent (Variables|Default|GetButtonHud))
  (Variables|Default|SetButtonHud 0))

(event OnSuccessed(ButtonHud)
  (Audio|PlaySound2D "/Game/Sounds/hl2beta/npc/cremator/alert_player.alert_player" 1.0 1.0 0.0 0 0)
  (Widget|RemovefromParent (Variables|Default|GetButtonHud))
  (Variables|Default|SetButtonHud 0))

(event Custom|OnInputFailed_Event
  (Audio|PlaySound2D "/Game/Retro_8Bit_Sounds/Retro_Orginal/Cues/retro_fail_sound_04_Cue.retro_fail_sound_04_Cue" 1.0 1.0 0.0 0 0)
  (Widget|RemovefromParent (Variables|Default|GetButtonHud))
  (Variables|Default|SetButtonHud 0))

(event Custom|OnInputSuccessed_Event
  (Audio|PlaySound2D "/Game/Sounds/hl2beta/npc/cremator/alert_player.alert_player" 1.0 1.0 0.0 0 0)
  (Widget|RemovefromParent (Variables|Default|GetButtonHud))
  (Variables|Default|SetButtonHud 0))

(event EventBeginPlay
  (|CallParentFunction) ; This node is disabled and will not be called.\nDrag off pins to build functionality.
)

(event Collision|EventActorBeginOverlap
  (params (OtherActor :type Actor%20Object%20Reference))
  (|CallParentFunction OtherActor) ; This node is disabled and will not be called.\nDrag off pins to build functionality.
)

(event EventTick
  (params (DeltaSeconds :type Float%20%28single-precision%29))
  (|CallParentFunction DeltaSeconds) ; This node is disabled and will not be called.\nDrag off pins to build functionality.
)

(event EventInteract
  (params (interactor :type Actor%20Object%20Reference) (interactedComponent :type Primitive%20Component%20Object%20Reference))
  (bind _returnvalue (UserInterface|CreateWidget "/Game/Blueprints/UI/CS/Keys/UMG_KeyPad.UMG_KeyPad_C" 0 (Variables|Default|GetNeededCode) self))
  (UserInterface|Viewport|AddtoViewport _returnvalue 0)
  (Variables|Default|SetButtonHud _returnvalue))

(fn ConstructionScript
  (|CallParentFunction))