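; Arena wave spawner that spawns AI soldiers from per-wave settings and announces wave progress through event dispatchers.
; SpawnNewWave creates rifle-armed soldiers at random spawn points, each possessed by a simulation AI controller and given AiTarget, or reports failure or no waves left.
; A looping CheckIfDead timer fires wave-finished and pauses once all spawned soldiers are dead, resuming after the next spawn.
; Setting InfiniteWaves skips spawning and reports no waves left.
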(event EventBeginPlay
  (bind _returnvalue (Utilities|Time|SetTimerbyFunctionName self "CheckIfDead" 0.1 true))
  (Variables|Default|SetUpdateTimerHandle _returnvalue))

(event Collision|EventActorBeginOverlap
  (params (OtherActor :type Actor%20Object%20Reference)))

(event EventTick
  (params (DeltaSeconds :type Float%20%28single-precision%29)))

(fn ConstructionScript)

(fn SpawnNewWave
  (bind _currentwaveid (Variables|WaveInfo|GetCurrentWaveId))
  (bind _wavesinfo (Variables|WaveInfo|GetWavesInfo))
  (bind _aitarget (Variables|AiSetup|GetAiTarget))
  (bind _output (Utilities|Array|Get(acopy) _wavesinfo _currentwaveid))
  (bind (_amounttospawn _spawnpointstouse) (Utilities|Struct|BreakS_WaveInfo _output))
  (bind _returnvalue (Utilities|Array|Length _spawnpointstouse))
  (bind _returnvalue_2 (- _returnvalue 1))
  (bind _returnvalue_3 (Math|Random|RandomIntegerinRange 0 _returnvalue_2))
  (bind _output_2 (Utilities|Array|Get(acopy) _spawnpointstouse _returnvalue_3))
  (bind _returnvalue_4 (Transformation|GetActorLocation _output_2))
  (bind _returnvalue_5 (Math|Transform|MakeTransform _returnvalue_4))
  (Utilities|Array|Clear (Variables|WaveInfo|GetSpawned))
  (if (and (not (Variables|WaveInfo|GetInfiniteWaves?)) (< _currentwaveid (Utilities|Array|Length _wavesinfo)))
    (if (> _returnvalue 0)
      (for _index (range 0 _amounttospawn)
        (bind _returnvalue_6 (Game|SpawnActorfromClass "/Game/Blueprints/CS/AI/AIC_SimulationController.AIC_SimulationController_C" _returnvalue_5 "Undefined" 0 5.0 0))
        (bind _returnvalue_7 (Game|SpawnActorfromClass "/Game/Blueprints/CS/AI/BP_SolderOld.BP_SolderOld_C" _returnvalue_5 "AdjustIfPossibleButAlwaysSpawn" 0 32.0 false true 0 false true false 35.0 _aitarget (Utilities|IsValid _aitarget) 0 2e+01 2e+01 "/Game/Blueprints/Weapons/BP_Rifle.BP_Rifle_C" true 6e+01 1.5e+03 2e+02 false 0))
        (Pawn|Possess _returnvalue_6 _returnvalue_7)
        (Default|UpdateWeapon _returnvalue_7)
        (Utilities|Array|Add (Variables|WaveInfo|GetSpawned) _returnvalue_7))
      (Default|CallOnFinishedSpawningWave)
      (Math|Integer|IncrementInt (Variables|WaveInfo|GetCurrentWaveId)
        (:%20%20
          (Utilities|Time|UnpauseTimerbyHandle (Variables|Default|GetUpdateTimerHandle))))
      (else
        (Default|CallOnFailedtoStartWave)))
    (else
      (Default|CallOnNoWavesLeft))))

(fn CheckifDead
  (for _array_element (Variables|WaveInfo|GetSpawned)
    (if (not (Variables|/Game/Blueprints/CS/AI/BP_SolderOld.BP_SolderOld_C|GetDead _array_element))
      (return)))
  (Default|CallOnWaveFinished)
  (Utilities|Time|PauseTimerbyHandle (Variables|Default|GetUpdateTimerHandle)))