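; Ladder actor that puts PropHunt characters into and out of ladder climbing.
; Entering the LadderCollision volume starts climbing on the character, unless it already overlaps TopTrigger.
; Leaving the volume stops climbing, with no TopTrigger check.
; Both events respond only to the overlapping capsule component, so weapon model and weapon collisions do not toggle climbing.
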(event OnComponentBeginOverlap(LadderCollision)
  (params (OverlappedComponent :type Primitive%20Component%20Object%20Reference) (OtherActor :type Actor%20Object%20Reference) (OtherComp :type Primitive%20Component%20Object%20Reference) (OtherBodyIndex :type Integer) (bFromSweep :type Boolean) (SweepResult :type Hit%20Result%20Structure%20%28by%20ref%29))
  (if (not (Collision|IsOverlappingActor (Variables|Default|GetTopTrigger) OtherActor :!class /Script/Engine.PrimitiveComponent))
    (bind _asprop_hunt_character (Utilities|Casting|CastToPropHuntCharacter OtherActor))
    ;[1 1 1] To prevent issues with both< weapon model and weapon collision
    (if (.bSuccess (Utilities|Casting|CastToCapsuleComponent OtherComp))
      (Class|PropHuntCharacter|StartClimbingLadder _asprop_hunt_character))))

(event OnComponentEndOverlap(LadderCollision)
  (params (OverlappedComponent :type Primitive%20Component%20Object%20Reference) (OtherActor :type Actor%20Object%20Reference) (OtherComp :type Primitive%20Component%20Object%20Reference) (OtherBodyIndex :type Integer))
  (bind _asprop_hunt_character (Utilities|Casting|CastToPropHuntCharacter OtherActor))
  (if (.bSuccess (Utilities|Casting|CastToCapsuleComponent OtherComp))
    (Class|PropHuntCharacter|StopClimbingLadder _asprop_hunt_character)))

(event EventBeginPlay)

(event Collision|EventActorBeginOverlap
  (params (OtherActor :type Actor%20Object%20Reference)))

(event EventTick
  (params (DeltaSeconds :type Float%20%28single-precision%29)))

(fn ConstructionScript)