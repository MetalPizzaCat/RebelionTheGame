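; Sliding door for a prop hunt game that toggles open and closed on interaction, or plays a lock sound when locked.
; A BP_Button can always interact with it, while a PropHuntCharacter can only when direct interaction is allowed.
; Open and Close restart an InterpToMovement component and a looping-until-stopped audio component, which halts with a stop sound when movement ends.
; Helper functions replace the movement control points or reverse and negate them.
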(event OnWaitBeginDelegate(InterpToMovement)
  (params (ImpactResult :type Hit%20Result%20Structure%20%28by%20ref%29) (Time :type Float%20%28single-precision%29)))

(event OnInterptoStop(InterpToMovement)
  (params (ImpactResult :type Hit%20Result%20Structure%20%28by%20ref%29) (Time :type Float%20%28single-precision%29))
  (Audio|PlaySoundatLocation (Variables|Default|GetStopSound) (Transformation|GetActorLocation) "0, 0, 0" 1.0 1.0 0.0 "/Game/SuperGrid/TutorialLevel/SoundEffects/Attenuation_Ambient.Attenuation_Ambient" 0 0)
  (Audio|Components|Audio|Stop (Variables|Default|GetAudio)))

(event EventBeginPlay
  (|CallParentFunction) ; This node is disabled and will not be called.\nDrag off pins to build functionality.
)

(event Collision|EventActorBeginOverlap
  (params (OtherActor :type Actor%20Object%20Reference))
  (|CallParentFunction OtherActor) ; This node is disabled and will not be called.\nDrag off pins to build functionality.
)

(event EventTick
  (params (DeltaSeconds :type Float%20%28single-precision%29))
  (|CallParentFunction DeltaSeconds) ; This node is disabled and will not be called.\nDrag off pins to build functionality.
)

(event EventInteract
  (params (interactor :type Actor%20Object%20Reference) (interactedComponent :type Primitive%20Component%20Object%20Reference))
  (Utilities|Casting|CastToPropHuntCharacter interactor
    (:then
      (if (Variables|Default|GetCanBeDirectlyInteracted)
        _
        (else
          (Utilities|Casting|CastToBP_Button interactor :!label _label))))
    (:CastFailed
      (goto _label)))
  (if (not (Variables|Default|GetLocked))
    (Audio|PlaySoundatLocation (Variables|Default|GetMovingSound) (Transformation|GetActorLocation) "0, 0, 0" 1.0 1.0 0.0 0 0 0)
    (if (Variables|Default|GetOpened)
      (CallFunction|Close)
      (else
        (CallFunction|Open)))
    (else
      (Audio|PlaySoundatLocation (Variables|Default|GetLockSound) (Transformation|GetActorLocation) "0, 0, 0" 1.0 1.0 0.0 0 0 0))))

(fn ConstructionScript
  (|CallParentFunction))

(fn Open
  (bind _interptomovement (Variables|Default|GetInterpToMovement))
  (if (Components|Activation|IsActive _interptomovement)
    _
    (else
      (Components|Activation|Activate _interptomovement false)))
  (|CallParentFunction)
  (Class|InterptoMovementComponent|RestartMovement (Variables|Default|GetInterpToMovement) 1.0)
  (Variables|Default|SetOpened true)
  (Audio|Components|Audio|Play (Variables|Default|GetAudio) 0.0))

(fn Close
  (bind _interptomovement (Variables|Default|GetInterpToMovement))
  (if (Components|Activation|IsActive _interptomovement)
    _
    (else
      (Components|Activation|Activate _interptomovement false)))
  (|CallParentFunction)
  (Class|InterptoMovementComponent|RestartMovement (Variables|Default|GetInterpToMovement) 1.0)
  (Variables|Default|SetOpened false)
  (Audio|Components|Audio|Play (Variables|Default|GetAudio) 0.0))

(fn ChangeControllPoints
  (params (Points :type Array%20of%20Interp%20Control%20Point%20Structures))
  (bind _interptomovement (Variables|Default|GetInterpToMovement))
  (Variables|/Script/Engine.InterpToMovementComponent|SetControlPoints _interptomovement Points)
  (Class|InterptoMovementComponent|FinaliseControlPoints _interptomovement))

(fn ReversePoints
  (bind _interptomovement (Variables|Default|GetInterpToMovement))
  (bind _arrayelement (Utilities|Array|ReverseforEachLoop (Variables|/Script/Engine.InterpToMovementComponent|GetControlPoints _interptomovement))
    (:LoopBody
      (Utilities|Array|Add (LocalVariables|Gettemp) (Utilities|Struct|MakeInterpControlPoint (Math|Vector|NegateVector (.PositionControlPoint (Utilities|Struct|BreakInterpControlPoint _arrayelement))) (.bPositionIsRelative (Utilities|Struct|BreakInterpControlPoint _arrayelement)))))
    (:Completed
      (Variables|/Script/Engine.InterpToMovementComponent|SetControlPoints _interptomovement (LocalVariables|Gettemp)))))