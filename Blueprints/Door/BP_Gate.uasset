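; BP_Gate is a gate actor with two toggled motions: partial opening, which yaws four gate panels, and full opening, which rolls six rotator parts.
; Looping timers step each motion, play sounds and flip its state flag when time runs out.
; Open works only while not fully opened, and GateFullOpen reverses a partial opening before starting the full motion.
; The construction script poses components from both flags.
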(event Custom|StartOpening_Event)

(event EventBeginPlay
  (|CallParentFunction) ; This node is disabled and will not be called.\nDrag off pins to build functionality.
)

(event Collision|EventActorBeginOverlap
  (params (OtherActor :type Actor%20Object%20Reference))
  (|CallParentFunction OtherActor) ; This node is disabled and will not be called.\nDrag off pins to build functionality.
)

(event EventTick
  (params (DeltaSeconds :type Float%20%28single-precision%29))
  (|CallParentFunction DeltaSeconds) ; This node is disabled and will not be called.\nDrag off pins to build functionality.
)

(fn ConstructionScript
  (bind _rotatorthingleft2 (Variables|Default|GetRotatorThingLeft2))
  (|CallParentFunction)
  (if (Variables|Default|GetOpened)
    (Transformation|SetRelativeRotation _rotatorthingleft2 "0, 0,90.000000" false false)
    (Transformation|SetRelativeRotation (Variables|Default|GetRotatorThingCenter2) "0,180.000000,270.000000" false false)
    (Transformation|SetRelativeRotation (Variables|Default|GetGateLeft1) "0,0.000000,180.000000" false false :!label _label)
    (Transformation|SetRelativeRotation (Variables|Default|GetGateRight2) "0,0.000000,180.000000" false false)
    (else
      (Transformation|SetRelativeRotation _rotatorthingleft2 "0, 0,180.000000" false false)
      (Transformation|SetRelativeRotation (Variables|Default|GetRotatorThingCenter1) "0,180.000000,360.000000" false false)
      (if (Variables|Default|GetPartiallyOpen)
        (Transformation|SetRelativeRotation (Variables|Default|GetGateLeft1) "0,90.000000,180.000000" false false)
        (Transformation|SetRelativeRotation (Variables|Default|GetGateRight2) "0,-90.000000,180.000000" false false)
        (else
          (goto _label))))))

(fn Open
  (|CallParentFunction)
  (if (and (not (Variables|Default|GetOpened)) (not (Utilities|Time|IsValidTimerHandle (Variables|Timer|GetMovementTimer))))
    (bind _returnvalue (Utilities|Time|SetTimerbyFunctionName self "ProccessOpening" 0.01 true))
    (Variables|Timer|SetMovementTimer _returnvalue)
    (Audio|Components|Audio|Play (Variables|Default|Getgate_move1) 0.0)))

(fn ProccessOpening
  (Transformation|SetRelativeRotation (Variables|Default|GetGateLeft1) (Math|Rotator|MakeRotator 1.8e+02 0.0 (* (- (select (Variables|Default|GetPartiallyOpen) -9e+01 0.0) (* -38.0 (Variables|Timer|GetTimePassed))) (select (Variables|Default|GetPartiallyOpen) -1.0 1.0))) false false)
  (Transformation|SetRelativeRotation (Variables|Default|GetGateLeft2) (Math|Rotator|MakeRotator 1.8e+02 0.0 (* (* (- (select (Variables|Default|GetPartiallyOpen) -9e+01 0.0) (* -38.0 (Variables|Timer|GetTimePassed))) (select (Variables|Default|GetPartiallyOpen) -1.0 1.0)) -1.0)) false false)
  (bind _output_get (Variables|Timer|SetTimePassed (+ (Variables|Timer|GetTimePassed) 0.01)))
  (if (>= _output_get (Variables|Timer|GetPartiallOpeningMovementTime))
    (Utilities|Time|ClearandInvalidateTimerbyHandle (Variables|Timer|GetMovementTimer))
    (Audio|Components|Audio|Play (Variables|Default|Getdoor_metal_large_chamber_close1) 0.0)
    (Variables|Default|SetPartiallyOpen (not (Variables|Default|GetPartiallyOpen)))
    (Variables|Timer|SetTimePassed 0.0)
    (if (Variables|Default|GetIsOpening)
      (CallFunction|GateFullOpen)
      (Variables|Default|SetIsOpening false))))

(fn GateFullOpen
  (if (not (Utilities|Time|IsValidTimerHandle (Variables|Timer|GetMovementTimer)))
    (if (Variables|Default|GetPartiallyOpen)
      (CallFunction|Open)
      (Variables|Default|SetIsOpening true)
      (else
        (bind _returnvalue (Utilities|Time|SetTimerbyFunctionName self "ProccessFullOpening" 0.01 true))
        (Variables|Timer|SetMovementTimer _returnvalue)
        (Audio|Components|Audio|Play (Variables|Default|GetMovementSound) 0.0)))))

(fn ProccessFullOpening
  (Transformation|AddRelativeRotation (Variables|Default|GetRotatorThingLeft2) (Math|Rotator|MakeRotator (* 0.1956 (select (Variables|Default|GetOpened) 1.0 -1.0)) 0.0 0.0) false false)
  (Transformation|AddRelativeRotation (Variables|Default|GetRotatorThingCenter2) (Math|Rotator|MakeRotator (* 0.1956 (select (Variables|Default|GetOpened) 1.0 -1.0)) 0.0 0.0) false false)
  (bind _output_get (Variables|Timer|SetTimePassed (+ (Variables|Timer|GetTimePassed) 0.01)))
  (if (>= _output_get (Variables|Timer|GetMovementTime))
    (Utilities|Time|ClearandInvalidateTimerbyHandle (Variables|Timer|GetMovementTimer))
    (Audio|Components|Audio|Play (Variables|Default|Getgarage_stop1) 0.0)
    (Variables|Default|SetOpened (not (Variables|Default|GetOpened)))
    (Variables|Timer|SetTimePassed 0.0)))