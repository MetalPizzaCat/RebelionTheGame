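; Base door Blueprint that provides open, close, lock and unlock functions, presumably for child doors to extend.
; Open, Close, Lock and UnLock only fire their matching event dispatchers, with no movement or state change.
; ToggleLocked calls Open or Close based on Opened rather than changing the lock, while ToggleOpen is empty.
; Health, key and save-component functions are stubs returning false or nothing, and the event graph is unused.
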(event EventBeginPlay)

(event Collision|EventActorBeginOverlap
  (params (OtherActor :type Actor%20Object%20Reference)))

(event EventTick
  (params (DeltaSeconds :type Float%20%28single-precision%29)))

(fn ConstructionScript)

(fn Open
  (Default|CallOnOpened))

(fn Close
  (Default|CallOnClosed))

(fn ToggleOpen)

(fn Lock
  (Default|CallOnLocked))

(fn UnLock
  (Default|CallOnUnLocked))

(fn ToggleLocked
  (if (Variables|Default|GetOpened)
    (CallFunction|Close)
    (else
      (CallFunction|Open))))

(fn AddHealth
  (params (amountOfHealth :type Float%20%28single-precision%29))
  (return false))

(fn ComponentstoSave
  (return 0))

(fn HasKeywithId
  (params (id :type Integer))
  (return false))

(fn RemoveKey
  (params (KeyId :type Integer))
  (return false))