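; Rotating door that players or AI can open, with optional locking by key ID and a debug key override.
; Interact checks the lock, then plays or reverses a timeline that drives mesh yaw, flipped by OpenInReverse, with movement, stop and locked sounds.
; An AI detection overlap triggers the soldier's door animation and opens the door after a short delay.
; Construction and load events set unlocked doors' rotation from the Opened state.
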(event OnComponentBeginOverlap(AiDetection)
  (params (OverlappedComponent :type Primitive%20Component%20Object%20Reference) (OtherActor :type Actor%20Object%20Reference) (OtherComp :type Primitive%20Component%20Object%20Reference) (OtherBodyIndex :type Integer) (bFromSweep :type Boolean) (SweepResult :type Hit%20Result%20Structure%20%28by%20ref%29))
  (if (Math|Boolean|ANDBoolean (Variables|Default|GetShouldAutoOpenForAI) (not (Variables|Default|GetOpened)) (not (Variables|Default|GetLocked)))
    (bind _asbp_solder_old (Utilities|Casting|CastToBP_SolderOld OtherActor)
      (:then
        (Class|BPIAnimBP|OpenDoorAnim(Message) _asbp_solder_old))
      (:CastFailed
        (bind _asbp_solder_physics_based (Utilities|Casting|CastToBP_SolderPhysicsBased OtherActor))
        (Class|BPIAI|StartOpeningDoor(Message) _asbp_solder_physics_based)))
    (Utilities|Time|SetTimerbyEvent (delegate Custom|AiOpen_Event) 0.7)))

(event Custom|AiOpen_Event
  (bind _returnvalue (Transformation|GetActorLocation))
  (bind _staticmesh (Variables|Default|GetStaticMesh))
  (bind _relativerotation (Variables|/Script/Engine.SceneComponent|GetRelativeRotation _staticmesh))
  (bind (_roll _pitch _yaw) (Math|Rotator|BreakRotator _relativerotation))
  (Audio|PlaySoundatLocation (Variables|Default|GetMovingSound) _returnvalue "0, 0, 0" 1.0 1.0 0.0 0 0 0)
  (if (Variables|Default|GetOpened)
    (bind _rotation (Timeline|DoorRotationTimeLine Reverse)
      (:Update
        (Transformation|SetRelativeRotation _staticmesh (Math|Rotator|MakeRotator _roll _pitch (* _rotation (Math|Float|SelectFloat -1.0 1.0 (Variables|Default|GetOpenInReverse)))) false false))
      (:Finished
        (Audio|PlaySoundatLocation (Variables|Default|GetStopSound) _returnvalue "0, 0, 0" 1.0 1.0 0.0 0 0 0)
        (Variables|Default|SetOpened (not (Variables|Default|GetOpened)))))
    (else
      (Timeline|DoorRotationTimeLine Play))))

(event Custom|ForceOpen_Event
  (bind _staticmesh (Variables|Default|GetStaticMesh))
  (bind _relativerotation (Variables|/Script/Engine.SceneComponent|GetRelativeRotation _staticmesh))
  (bind (_roll _pitch _yaw) (Math|Rotator|BreakRotator _relativerotation))
  (bind _rotation (Timeline|DoorRotationTimeLine Play)
    (:Update
      (Transformation|SetRelativeRotation _staticmesh (Math|Rotator|MakeRotator _roll _pitch (* _rotation (Math|Float|SelectFloat -1.0 1.0 (Variables|Default|GetOpenInReverse)))) false false))
    (:Finished
      (Audio|PlaySoundatLocation (Variables|Default|GetStopSound) (Transformation|GetActorLocation) "0, 0, 0" 1.0 1.0 0.0 0 0 0)
      (Variables|Default|SetOpened (not (Variables|Default|GetOpened))))))

(event Custom|ForceClose_Event
  (bind _staticmesh (Variables|Default|GetStaticMesh))
  (bind _relativerotation (Variables|/Script/Engine.SceneComponent|GetRelativeRotation _staticmesh))
  (bind (_roll _pitch _yaw) (Math|Rotator|BreakRotator _relativerotation))
  (bind _rotation (Timeline|DoorRotationTimeLine Reverse)
    (:Update
      (Transformation|SetRelativeRotation _staticmesh (Math|Rotator|MakeRotator _roll _pitch (* _rotation (Math|Float|SelectFloat -1.0 1.0 (Variables|Default|GetOpenInReverse)))) false false))
    (:Finished
      (Audio|PlaySoundatLocation (Variables|Default|GetStopSound) (Transformation|GetActorLocation) "0, 0, 0" 1.0 1.0 0.0 0 0 0)
      (Variables|Default|SetOpened (not (Variables|Default|GetOpened))))))

(event EventBeginPlay
  (|CallParentFunction) ; This node is disabled and will not be called.\nDrag off pins to build functionality.
)

(event Collision|EventActorBeginOverlap
  (params (OtherActor :type Actor%20Object%20Reference))
  (|CallParentFunction OtherActor) ; This node is disabled and will not be called.\nDrag off pins to build functionality.
)

(event EventTick
  (params (DeltaSeconds :type Float%20%28single-precision%29))
  (|CallParentFunction DeltaSeconds) ; This node is disabled and will not be called.\nDrag off pins to build functionality.
)

(event EventInteract
  (params (interactor :type Actor%20Object%20Reference) (interactedComponent :type Primitive%20Component%20Object%20Reference))
  (bind _returnvalue (Transformation|GetActorLocation))
  (bind _staticmesh (Variables|Default|GetStaticMesh))
  (bind _relativerotation (Variables|/Script/Engine.SceneComponent|GetRelativeRotation _staticmesh))
  (bind (_roll _pitch _yaw) (Math|Rotator|BreakRotator _relativerotation))
  (if (Variables|Default|GetLocked)
    (if (Variables|Default|GetCanBeOpenedWithKey)
      (bind _returnvalue_2 (Class|InteractionInterface|HasKeywithId(Message) interactor (Variables|Default|GetKeyId)))
      (bind _returnvalue_3 (Class|InteractionInterface|HasKeywithId(Message) interactor -1)) ; -1 is id for debug key, DOES NOT ALLOWED TO BE PICKED UP BY PLAYER IN NORMAL GAME
      (if (or _returnvalue_2 _returnvalue_3)
        (Audio|PlaySoundatLocation (Variables|Default|GetMovingSound) _returnvalue "0, 0, 0" 1.0 1.0 0.0 0 0 0 :!label _label)
        (if (Variables|Default|GetOpened)
          (bind _rotation (Timeline|DoorRotationTimeLine Reverse)
            (:Update
              (Transformation|SetRelativeRotation _staticmesh (Math|Rotator|MakeRotator _roll _pitch (* _rotation (Math|Float|SelectFloat -1.0 1.0 (Variables|Default|GetOpenInReverse)))) false false))
            (:Finished
              (Audio|PlaySoundatLocation (Variables|Default|GetStopSound) _returnvalue "0, 0, 0" 1.0 1.0 0.0 0 0 0)
              (Variables|Default|SetOpened (not (Variables|Default|GetOpened)))))
          (else
            (Timeline|DoorRotationTimeLine Play)))
        (else
          (Audio|PlaySoundatLocation (Variables|Default|GetLockSound) (Transformation|GetActorLocation) "0, 0, 0" 1.0 1.0 0.0 0 0 0 :!label _label_2)))
      (else
        (goto _label_2)))
    (else
      (goto _label))))

(event EventActorLoaded
  (bind _staticmesh (Variables|Default|GetStaticMesh))
  (bind _relativerotation (Variables|/Script/Engine.SceneComponent|GetRelativeRotation _staticmesh))
  (bind (_roll _pitch) (Math|Rotator|BreakRotator _relativerotation))
  (if (not (Variables|Default|GetLocked))
    (Transformation|SetRelativeRotation _staticmesh (Math|Rotator|MakeRotator _roll _pitch (Math|Float|SelectFloat (Math|Float|SelectFloat -9e+01 9e+01 (Variables|Default|GetOpenInReverse)) 0.0 (Variables|Default|GetOpened))) false false)))

(fn ConstructionScript
  (bind _staticmesh (Variables|Default|GetStaticMesh))
  (bind _relativerotation (Variables|/Script/Engine.SceneComponent|GetRelativeRotation _staticmesh))
  (bind (_roll _pitch) (Math|Rotator|BreakRotator _relativerotation))
  (|CallParentFunction)
  (if (not (Variables|Default|GetLocked))
    (Transformation|SetRelativeRotation _staticmesh (Math|Rotator|MakeRotator _roll _pitch (Math|Float|SelectFloat 9e+01 0.0 (Variables|Default|GetOpened))) false false)))

(fn Open
  (|CallParentFunction))

(fn Lock
  (|CallParentFunction))

(fn Close
  (|CallParentFunction))

(fn UnLock
  (|CallParentFunction))

(fn ComponentstoSave
  (return 0))