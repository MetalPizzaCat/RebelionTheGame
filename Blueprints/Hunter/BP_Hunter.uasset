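; First-person Hunter player character that shoots, aims, reloads, swaps between two rifles and takes damage, with a HUD widget.
; The weapon is a child actor that handles firing; a looping timer polls the held fire button for automatic weapons.
; State getters expose aiming, firing and reloading, with most others stubbed, and a notify event refills the clip.
; Damage reduces health until death ragdolls the body and unpossesses the controller.
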(event Custom|Shoot_Event
  (bind _asweapon_base (Utilities|GetWeapon))
  (bind _weaponbase (Variables|Default|GetWeaponBase))
  (bind _childactor (Variables|/Script/Engine.ChildActorComponent|GetChildActor _weaponbase))
  (bind _asweapon_base_2 (Utilities|Casting|CastToWeaponBase _childactor))
  ;[1 1 1] Continues fire
  (Utilities|IsValid _asweapon_base
    (:Is%20Valid
      (if (Utilities|Enum|Equal(Enum) (Variables|/Script/PropHunt.WeaponBase|GetShootingType _asweapon_base) "EAT_Auto")
        (if (Variables|Default|GetFireButtonPressed)
          (if (not (Variables|Default|GetFiring))
            (Utilities|IsValid _asweapon_base_2
              (:Is%20Valid
                (bind _returnvalue (Class|WeaponBase|PrimaryFire _asweapon_base_2 (Transformation|GetSocketLocation (Variables|/Script/PropHunt.WeaponBase|GetWeaponMesh (Utilities|GetWeapon)) "b_gun_muzzleflash") (Transformation|GetWorldRotation (Variables|Default|GetFirstPersonCameraComponent))))
                (if _returnvalue
                  (Variables|Default|SetFiring true)
                  (elif (<= (Variables|/Script/PropHunt.WeaponBase|GetAmmoInTheClip _asweapon_base_2) 0)
                    (Audio|PlaySoundatLocation (Variables|/Script/PropHunt.WeaponBase|GetPrimaryOutOfAmmoSound _asweapon_base_2) (Transformation|GetActorLocation) "0, 0, 0" 1.0 1.0 0.0 0 0 0)))))))))))

(event Custom|Test_SpawnBullet_Event
  (Game|SpawnActorfromClass (Variables|TEMP|GetTemp_ProjClass) (Math|Transform|MakeTransform (Variables|TEMP|GetTemp_Loc) (Variables|TEMP|GetTem_Rot)) "Undefined" 0 0))

(event EventBeginPlay
  (bind _asweapon_base (Utilities|GetWeapon))
  (bind _self self)
  ;[1 1 1] Begin Play
  (Utilities|IsValid _asweapon_base
    (:Is%20Valid
      (Class|WeaponBase|SetOnwerPlayer _asweapon_base _self))
    (:Is%20Not%20Valid
      _))
  (bind _returnvalue (UserInterface|CreateWidget "/Game/Blueprints/UI/PropHunt/UMG_HunterHud.UMG_HunterHud_C" 0 _self))
  (bind _output_get (Variables|Default|SetUMG_HunterHUD _returnvalue))
  (UserInterface|Viewport|AddtoViewport _output_get 0)
  (Transformation|AttachComponentToComponent (Variables|Default|GetFP_Gun) (Variables|Character|GetMesh) "GripPoint" "KeepRelative" "KeepRelative" "KeepRelative" true)
  (Class|SkinnedMeshComponent|SetSkeletalMesh (Variables|Default|GetMP_Gun) (Variables|/Script/Engine.SkinnedMeshComponent|GetSkeletalMesh (Variables|/Script/PropHunt.WeaponBase|GetWeaponMesh _asweapon_base)) true)
  (bind _returnvalue_2 (Utilities|Time|SetTimerbyEvent (delegate Custom|Shoot_Event) 0.01 true))
  (Variables|Default|SetShootingTimerHandle _returnvalue_2))

(event EventSetIsShooting
  (params (is :type Boolean))
  ;[1 1 1] Update is Firing
  (Variables|Default|SetFiring is))

(event EventNotifyEndReload
  (bind _asweapon_base (Utilities|GetWeapon))
  ;[1 1 1] End reload
  (Utilities|IsValid _asweapon_base
    (:Is%20Valid
      (Variables|/Script/PropHunt.WeaponBase|SetAmmoInTheClip _asweapon_base (Variables|/Script/PropHunt.WeaponBase|GetDefaultAmmoInTheClip _asweapon_base))
      (Variables|Default|SetReloading false))
    (:Is%20Not%20Valid
      (Variables|Default|SetReloading false))))

(event Game|Damage|EventAnyDamage
  (params (Damage :type Float%20%28single-precision%29) (DamageType :type Damage%20Type%20Object%20Reference) (InstigatedBy :type Controller%20Object%20Reference) (DamageCauser :type Actor%20Object%20Reference))
  ;[1 1 1] On any damage
  (Audio|PlaySoundatLocation "/Game/Sounds/hl2/physics/flesh/flesh_impact_bullet_Cue.flesh_impact_bullet_Cue" (Transformation|GetActorLocation) "0, 0, 0" 1.0 1.0 0.0 0 0 0)
  (bind _output_get (Variables|Default|SetHealth (- (Variables|Default|GetHealth) Damage)))
  (if (<= _output_get 0.0)
    (CallFunction|Die)))

(event EventRequestSpawnProjectile
  (params (ProjectileClass :type Prop%20Hunt%20Projectile%20Class%20Reference) (location :type Vector :default "0, 0, 0") (rotation :type Rotator :default "0, 0, 0"))
  (Variables|TEMP|SetTemp_ProjClass ProjectileClass)
  (Variables|TEMP|SetTem_Rot rotation)
  (Variables|TEMP|SetTemp_Loc location))

(event Input|ActionEvents|InputActionAim
  (params (Key :type Key%20Structure))
  ;[1 1 1] Aim
  (:Pressed
    (Variables|Default|SetAiming true))
  (:Released
    (Variables|Default|SetAiming false)))

(event Input|ActionEvents|InputActionFire
  (params (Key :type Key%20Structure))
  (bind _weaponbase (Variables|Default|GetWeaponBase))
  (bind _childactor (Variables|/Script/Engine.ChildActorComponent|GetChildActor _weaponbase))
  (bind _asweapon_base (Utilities|Casting|CastToWeaponBase _childactor))
  ;[1 1 1] Shoot
  (:Pressed
    (Variables|Default|SetFireButtonPressed true)
    (if (not (Variables|Default|GetFiring))
      (Utilities|IsValid _asweapon_base
        (:Is%20Valid
          (bind _returnvalue (Class|WeaponBase|PrimaryFire _asweapon_base (Transformation|GetSocketLocation (Variables|/Script/PropHunt.WeaponBase|GetWeaponMesh (Utilities|GetWeapon)) "b_gun_muzzleflash") (Transformation|GetWorldRotation (Variables|Default|GetFirstPersonCameraComponent))))
          (if _returnvalue
            (Variables|Default|SetFiring true)
            (elif (and (<= (Variables|/Script/PropHunt.WeaponBase|GetAmmoInTheClip _asweapon_base) 0) (Variables|/Script/PropHunt.WeaponBase|GetbCanShoot _asweapon_base))
              (Audio|PlaySoundatLocation (Variables|/Script/PropHunt.WeaponBase|GetPrimaryOutOfAmmoSound _asweapon_base) (Transformation|GetActorLocation) "0, 0, 0" 1.0 1.0 0.0 0 0 0)))))))
  (:Released
    (Variables|Default|SetFireButtonPressed false)))

(event Input|ActionEvents|InputActionReload
  (params (Key :type Key%20Structure))
  (bind _asweapon_base (Utilities|GetWeapon))
  ;[1 1 1] Ask to reload
  (:Pressed
    (if (not (Variables|Default|GetReloading))
      (Utilities|IsValid _asweapon_base
        (:Is%20Valid
          (if (< (Variables|/Script/PropHunt.WeaponBase|GetAmmoInTheClip _asweapon_base) (Variables|/Script/PropHunt.WeaponBase|GetDefaultAmmoInTheClip _asweapon_base))
            (Variables|Default|SetReloading true)))))))

(event Input|KeyboardEvents|1
  (params (Key :type Key%20Structure))
  (:Pressed
    (CallFunction|ChangeWeapon "/Game/Blueprints/Weapons/BP_Rifle.BP_Rifle_C")))

(event Input|KeyboardEvents|2
  (params (Key :type Key%20Structure))
  (:Pressed
    (CallFunction|ChangeWeapon "/Game/Blueprints/Weapons/BP_Rifle_AK47.BP_Rifle_AK47_C")))

(fn ConstructionScript
  (bind _mesh (Variables|Character|GetMesh))
  (Class|PrimitiveComponent|SetOwnerNoSee (Variables|Default|GetSkeletalMesh) true)
  (Transformation|SetRelativeRotation _mesh "0,-90.000000, 0" false false)
  (Components|SkinnedMesh|HideBonebyName _mesh (Variables|Default|GetHeadBoneName) "PBO_None")
  (Transformation|AttachComponentToComponent _mesh (Variables|Default|GetFirstPersonCameraComponent) "None" "KeepRelative" "KeepRelative" "KeepRelative" true)
  (Components|SkinnedMesh|HideBonebyName _mesh "pelvis" "PBO_None")
  (Transformation|AttachComponentToComponent (Variables|Default|GetMP_Gun) (Variables|Default|GetSkeletalMesh) "GripPoint" "KeepRelative" "KeepRelative" "KeepRelative" true))

(fn ChangeWeapon
  (params (NewWeaponClass :type Weapon%20Base%20Class%20Reference))
  (ChildActorComponent|SetChildActorClass (Variables|Default|GetWeaponBase) NewWeaponClass)
  (Class|WeaponBase|SetOnwerPlayer (Utilities|GetWeapon) self))

(fn Die
  (Physics|SetSimulatePhysics (Variables|Default|GetSkeletalMesh) true)
  (Collision|SetCollisionEnabled (Variables|Default|GetSkeletalMesh) "QueryAndPhysics")
  (bind _asplayer_controller (Utilities|Casting|CastToPlayerController (Pawn|GetController)))
  (Pawn|UnPossess _asplayer_controller)
  (Collision|SetCollisionEnabled (Variables|Default|GetCapsuleComponent) "NoCollision")
  (return true))

(fn GetFinishedReload
  (return false))

(fn GetIsAiming
  (return (Variables|Default|GetAiming)))

(fn GetIsDead
  (return false))

(fn GetIsHurtAnimPlaying
  (return false))

(fn GetIsIdle
  (return false))

(fn GetIsinFight
  (return false))

(fn GetIsReloading
  (return (Variables|Default|GetReloading)))

(fn GetIsShooting
  (return (Variables|Default|GetFiring)))

(fn GetIsSprinting
  (return false))

(fn GetIsSwitchingWeapon
  (return false))

(fn GetIsWeaponHolstered
  (return false))

(fn GetLeftFootOffset
  (return 0.0))

(fn GetRightFootOffset
  (return 0.0))

(fn GetWeaponAnimationType
  (return "EAT_Rifle"))

(fn IsMelee
  (return false))

(fn IsOpeningDoor
  (return false))

(fn IsSprinting
  (return false))

(fn PickupWeapon
  (params (weaponClass :type Weapon%20Base%20Class%20Reference) (ammoInTheClip :type Integer))
  (return false))

(fn ShouldContinueReloading
  (return false))