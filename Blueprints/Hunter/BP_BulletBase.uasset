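; Base projectile for Hunter bullets that damages what it hits and leaves surface-specific impact effects.
; On hit it pushes simulating physics objects, applies generic damage to PropCharacters or point damage to others, then destroys itself.
; Particles, sound and a random decal come from DT_BulletHitEffects by physical surface, matched on AlternativeName in packaged builds, with a Default fallback.
; Overlaps call ImpactAtLocation with velocity-scaled power.
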(event OnComponentHit(CollisionComp)
  (params (HitComponent :type Primitive%20Component%20Object%20Reference) (OtherActor :type Actor%20Object%20Reference) (OtherComp :type Primitive%20Component%20Object%20Reference) (NormalImpulse :type Vector :default "0, 0, 0") (Hit :type Hit%20Result%20Structure%20%28by%20ref%29)))

(event OnComponentBeginOverlap(CollisionComp)
  (params (OverlappedComponent :type Primitive%20Component%20Object%20Reference) (OtherActor :type Actor%20Object%20Reference) (OtherComp :type Primitive%20Component%20Object%20Reference) (OtherBodyIndex :type Integer) (bFromSweep :type Boolean) (SweepResult :type Hit%20Result%20Structure%20%28by%20ref%29))
  (CallFunction|ImpactatLocation (.Location (Collision|BreakHitResult SweepResult)) 5.0 (/ (Math|Vector|VectorLength (Transformation|GetVelocity)) 2e+03)))

(event Collision|EventHit
  (params (MyComp :type Primitive%20Component%20Object%20Reference) (Other :type Actor%20Object%20Reference) (OtherComp :type Primitive%20Component%20Object%20Reference) (bSelfMoved :type Boolean) (HitLocation :type Vector :default "0, 0, 0") (HitNormal :type Vector :default "0, 0, 0") (NormalImpulse :type Vector :default "0, 0, 0") (Hit :type Hit%20Result%20Structure%20%28by%20ref%29))
  (bind (_bblockinghit _binitialoverlap _time _distance _location _impactpoint _normal _impactnormal _physmat _hitactor _hitcomponent _hitbonename _hititem _faceindex _tracestart) (Collision|BreakHitResult Hit))
  (bind _self self)
  (bind _damage (Variables|Default|GetDamage))
  (bind _startlocation (Variables|Default|GetStartLocation))
  (bind _startlocation_2 (Variables|Default|GetStartLocation))
  (bind _returnvalue (Math|Rotator|FindLookatRotation _startlocation_2 _location))
  (bind _returnvalue_2 (Math|Rotator|FindLookatRotation _startlocation _location))
  (bind _surfacetype (Variables|/Script/Engine.PhysicalMaterial|GetSurfaceType _physmat))
  (bind _hiteffects (CallFunction|GetBulletHitEffect _surfacetype))
  (bind (_sound _particleeffect _decalmaterial) (Utilities|Struct|BreakS_BulletHitEffect _hiteffects))
  (if (!= Other (Components|GetOwner))
    (if (Math|Boolean|ANDBoolean (!= Other self) (Utilities|IsValid Other) (Physics|IsSimulatingPhysics OtherComp "None"))
      (Physics|AddImpulseatLocation OtherComp (* (Transformation|GetVelocity) (Variables|Default|GetImpluseMultiplier)) HitLocation "None"))
    (Utilities|Casting|CastToPropCharacter Other
      (:then
        (Game|Damage|ApplyDamage Other (Variables|Default|GetDamage) 0 _self "/Script/Engine.DamageType"))
      (:CastFailed
        (bind _asbp_cscharacter (Utilities|Casting|CastToBP_CSCharacter Other)
          (:then
            (Game|Damage|ApplyPointDamage _asbp_cscharacter _damage _tracestart Hit 0 _self "/Script/Engine.DamageType"))
          (:CastFailed
            (Game|Damage|ApplyPointDamage Other _damage _tracestart Hit 0 _self "/Script/Engine.DamageType")))))
    (Utilities|IsValid _physmat
      (:Is%20Valid
        (Effects|SpawnEmitteratLocation _particleeffect _location _returnvalue)
        (Audio|PlaySoundatLocation _sound _location "0, 0, 0" 1.0 1.0 0.0 0 0 0)
        (bind _returnvalue_3 (Class|GameplayStatics|SpawnDecalAttached (Utilities|Array|Get(acopy) _decalmaterial (Math|Random|RandomInteger (- (Utilities|Array|Length _decalmaterial) 1))) "2.000000,6.000000,6.000000" _hitcomponent "None" _location _returnvalue "KeepWorldPosition" 0.0))
        (Rendering|Components|Decal|SetFadeScreenSize _returnvalue_3 0.001))
      (:Is%20Not%20Valid
        (bind _returnvalue_4 (Utilities|GetDataTableRow "/Game/DataTable/DT_BulletHitEffects.DT_BulletHitEffects" "Default")
          (:then
            (Effects|SpawnEmitteratLocation (.ParticleEffect (Utilities|Struct|BreakS_BulletHitEffect _returnvalue_4)) _location _returnvalue_2)
            (Audio|PlaySoundatLocation (.Sound (Utilities|Struct|BreakS_BulletHitEffect _returnvalue_4)) _location "0, 0, 0" 1.0 1.0 0.0 0 0 0)
            (bind _returnvalue_5 (Class|GameplayStatics|SpawnDecalAttached (Utilities|Array|Get(acopy) (.DecalMaterial (Utilities|Struct|BreakS_BulletHitEffect _returnvalue_4)) (Math|Random|RandomInteger (- (Utilities|Array|Length (.DecalMaterial (Utilities|Struct|BreakS_BulletHitEffect _returnvalue_4))) 1))) "2.000000,6.000000,6.000000" _hitcomponent "None" _location _returnvalue_2 "KeepWorldPosition" 0.0))
            (Rendering|Components|Decal|SetFadeScreenSize _returnvalue_5 0.001)))))
    (Actor|DestroyActor)))

(fn ConstructionScript)

(fn GetBulletHitEffect
  (params (SurfaceType :type EPhysicalSurface%20Enum :default "SurfaceType_Default"))
  (bind _returnvalue (Utilities|String|EnumtoString SurfaceType))
  (if (Class|KismetSystemLibrary|IsPackagedforDistribution)
    (bind _outrownames (DataTable|GetDataTableRowNames "/Game/DataTable/DT_BulletHitEffects.DT_BulletHitEffects"))
    (for _array_element _outrownames
      (bind _returnvalue_2 (Utilities|GetDataTableRow "/Game/DataTable/DT_BulletHitEffects.DT_BulletHitEffects" _array_element)
        (:then
          (if (Utilities|Enum|Equal(Enum) (.AlternativeName (Utilities|Struct|BreakS_BulletHitEffect _returnvalue_2)) _returnvalue)
            (return _returnvalue_2)))))
    (else
      (bind _returnvalue_3 (Utilities|GetDataTableRow "/Game/DataTable/DT_BulletHitEffects.DT_BulletHitEffects" (Utilities|String|StringToName _returnvalue))
        (:then
          (return _returnvalue_3))
        (:RowNotFound
          _))))
  (bind _returnvalue_4 (Utilities|GetDataTableRow "/Game/DataTable/DT_BulletHitEffects.DT_BulletHitEffects" "Default")
    (:then
      (return _returnvalue_4))))