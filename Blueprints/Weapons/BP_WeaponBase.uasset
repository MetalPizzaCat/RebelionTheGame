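; Base weapon Blueprint that handles mesh visibility, pickup collision, firing noise and destruction tracking.
; The construction script makes pickup weapons visible and collidable, while others have no collision and follow their visibility flag.
; Primary fire effects make noise at the muzzle socket through the owner.
; On BeginPlay it finds the level's BP_DestroyedActorManager, where a pickup weapon records its display name when destroyed.
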(event EventBeginPlay
  ;[1 1 1] Find Destroyed Actors Manager
  (bind _outactors (Actor|GetAllActorsOfClass "/Game/Blueprints/SaveSystem/BP_DestroyedActorManager.BP_DestroyedActorManager_C"))
  (Utilities|IsValid (Utilities|Array|Get(acopy) _outactors)
    (:Is%20Valid
      (Variables|SaveSystem|SetDestroyedActorManager (Utilities|Array|Get(acopy) _outactors)))
    (:Is%20Not%20Valid
      (Development|PrintString "ERROR: Failed to find DestroyedActorsManager. Please add one to the world" true true "(R=1.000000,G=0.010000,B=0.031000,A=1.000000)" 1e+01))))

(event Collision|EventActorBeginOverlap
  (params (OtherActor :type Actor%20Object%20Reference)))

(event EventTick
  (params (DeltaSeconds :type Float%20%28single-precision%29)))

(event EventPrimaryFireEffects
  (params (location :type Vector :default "0, 0, 0") (rotation :type Rotator :default "0, 0, 0"))
  (Class|Actor|MakeNoise (Variables|Default|GetWeaponOwner) 1.0 0 (Transformation|GetSocketLocation (Variables|Default|GetWeaponMesh) "MuzzleSocket") 4.2e+03 "None"))

(event EventDestroyed
  (bind _destroyedactormanager (Variables|SaveSystem|GetDestroyedActorManager))
  (Utilities|IsValid _destroyedactormanager
    (:Is%20Valid
      (if (Variables|Default|GetbCanBePickedUp)
        (Utilities|Array|Add (Variables|/Game/Blueprints/SaveSystem/BP_DestroyedActorManager.BP_DestroyedActorManager_C|GetActors _destroyedactormanager) (Utilities|GetDisplayName self))))))

(fn ConstructionScript
  (bind _weaponmesh (Variables|Default|GetWeaponMesh))
  (bind _weaponmesh_2 (Variables|Default|GetWeaponMesh))
  (Rendering|SetVisibility _weaponmesh_2 (Variables|Visibility|GetShouldBeVisible) false)
  (if (Variables|Default|GetbCanBePickedUp)
    (Collision|SetCollisionEnabled _weaponmesh "QueryAndPhysics")
    (Rendering|SetVisibility _weaponmesh_2 true false)
    (else
      (Collision|SetCollisionEnabled _weaponmesh "NoCollision"))))

(fn UpdateVisibility
  (params (New :type Boolean))
  (Rendering|SetVisibility (Variables|Default|GetWeaponMesh) New false))

(fn GetWeaponEffectsSocketLocation
  (return (Transformation|GetSocketLocation (Variables|Default|GetWeaponMesh) (Utilities|String|StringToName (Variables|Default|GetWeaponEffectsSocketName)))))