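; BP_SniperRifle is a sniper rifle weapon Blueprint that supplies the cosmetic and noise response to primary fire.
; Its PrimaryFireEffects event plays the fire sound with ambient attenuation and spawns the assault rifle's muzzle flash at the given location.
; It then makes the weapon owner emit a range-limited noise there.
; The Blueprint holds no firing logic, and its construction script only calls the parent.
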(event EventBeginPlay
  (|CallParentFunction) ; This node is disabled and will not be called.\nDrag off pins to build functionality.
)

(event Collision|EventActorBeginOverlap
  (params (OtherActor :type Actor%20Object%20Reference))
  (|CallParentFunction OtherActor) ; This node is disabled and will not be called.\nDrag off pins to build functionality.
)

(event EventTick
  (params (DeltaSeconds :type Float%20%28single-precision%29))
  (|CallParentFunction DeltaSeconds) ; This node is disabled and will not be called.\nDrag off pins to build functionality.
)

(event EventPrimaryFireEffects
  (params (location :type Vector :default "0, 0, 0") (rotation :type Rotator :default "0, 0, 0"))
  (Audio|PlaySoundatLocation (Variables|Default|GetPrimaryFireSound) location "0, 0, 0" 1.0 1.0 0.0 "/Game/SuperGrid/TutorialLevel/SoundEffects/Attenuation_Ambient.Attenuation_Ambient" 0 0)
  (Effects|SpawnEmitteratLocation "/Game/MilitaryWeapDark/FX/P_AssaultRifle_MuzzleFlash.P_AssaultRifle_MuzzleFlash" location rotation)
  (Class|Actor|MakeNoise (Variables|Default|GetWeaponOwner) 1.0 0 location 1.8e+03 "None"))

(fn ConstructionScript
  (|CallParentFunction))