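; Base grenade actor that explodes on a timer started at BeginPlay.
; Explode spawns the particle effect, decal and sound, applies radial damage with falloff around itself, then destroys the actor.
; The decal comes from a short trace along the actor's down vector, using the hit surface type as a row name in DT_ExplosionDecalInfo.
; It picks a random material from that row, falling back to the Default row.
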(event Collision|EventActorBeginOverlap
  (params (OtherActor :type Actor%20Object%20Reference))
  (|CallParentFunction OtherActor) ; This node is disabled and will not be called.\nDrag off pins to build functionality.
)

(event EventTick
  (params (DeltaSeconds :type Float%20%28single-precision%29))
  (|CallParentFunction DeltaSeconds) ; This node is disabled and will not be called.\nDrag off pins to build functionality.
)

(event EventBeginPlay
  (bind _returnvalue (Utilities|Time|SetTimerbyFunctionName self "Explode" (Variables|Default|GetExplosionTime)))
  (Variables|Default|SetExplosionTimerHandle _returnvalue))

(fn ConstructionScript
  (|CallParentFunction))

(fn Explode
  (bind _returnvalue (Transformation|GetActorLocation))
  (bind _self self)
  (bind _basedamage (Variables|Default|GetBaseDamage))
  (bind _damageradius (Variables|Default|GetDamageRadius))
  (Effects|SpawnEmitteratLocation (Variables|Default|GetExplosionEffect) _returnvalue)
  (CallFunction|SpawnExplosionDecal)
  (Audio|PlaySoundatLocation (Variables|Default|GetExplosionSound) _returnvalue "0, 0, 0" 1.0 1.0 0.0 "/Game/SuperGrid/TutorialLevel/SoundEffects/Attenuation_Ambient.Attenuation_Ambient" 0 0)
  (Class|GameplayStatics|ApplyRadialDamagewithFalloff _basedamage (* _basedamage 0.2) (Transformation|GetActorLocation) (* _damageradius 0.8) _damageradius 1.0 (Variables|Default|GetDamageType) (Utilities|Array|MakeArray _self) _self 0 "ECC_Visibility")
  (Actor|DestroyActor))

(fn SpawnExplosionDecal
  (bind _returnvalue (Transformation|GetActorLocation))
  (bind (_outhit _returnvalue_2) (Collision|LineTraceByChannel _returnvalue (+ _returnvalue (* (Transformation|GetActorUpVector) -1e+01)) "TraceTypeQuery1" false 0 "None"))
  (if _returnvalue_2
    (bind _returnvalue_3 (Utilities|GetDataTableRow "/Game/DataTable/DT_ExplosionDecalInfo.DT_ExplosionDecalInfo" (Utilities|String|StringToName (Utilities|String|EnumtoString (Variables|/Script/Engine.PhysicalMaterial|GetSurfaceType (.PhysMat (Collision|BreakHitResult _outhit))))))
      (:then
        (Rendering|Decal|SpawnDecalatLocation (Utilities|Array|Get(acopy) (.ExplosionDecal (Utilities|Struct|BreakS_PhysMatExplosionDecalsInfo _returnvalue_3)) (Math|Random|RandomIntegerinRange 0 (- (Utilities|Array|Length (.ExplosionDecal (Utilities|Struct|BreakS_PhysMatExplosionDecalsInfo _returnvalue_3))) 1))) "10.000000,100.000000,100.000000" _returnvalue "-90.000000,0.000000,0.000000" 0.0))
      (:RowNotFound
        (bind _returnvalue_4 (Utilities|GetDataTableRow "/Game/DataTable/DT_ExplosionDecalInfo.DT_ExplosionDecalInfo" "Default")
          (:then
            (Rendering|Decal|SpawnDecalatLocation (Utilities|Array|Get(acopy) (.ExplosionDecal (Utilities|Struct|BreakS_PhysMatExplosionDecalsInfo _returnvalue_4)) (Math|Random|RandomIntegerinRange 0 (- (Utilities|Array|Length (.ExplosionDecal (Utilities|Struct|BreakS_PhysMatExplosionDecalsInfo _returnvalue_4))) 1))) "10.000000,100.000000,100.000000" _returnvalue "-90.000000,0.000000,0.000000" 0.0)))))))

(fn ComponentstoSave
  (return 0))