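; Base melee weapon Blueprint that provides a cooldown-gated primary fire and a short-range hit attack.
; PrimaryFire only starts the EndCooldown timer and returns true, without calling its parent or Attack.
; Attack runs a debug-drawn forward line trace on Visibility and applies point damage on a hit.
; It picks particle, sound and random attached decal from DT_BulletHitEffects by surface type, falling back to the Default row.
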(event EventBeginPlay
  (|CallParentFunction) ; This node is disabled and will not be called.\nDrag off pins to build functionality.
)

(event Collision|EventActorBeginOverlap
  (params (OtherActor :type Actor%20Object%20Reference))
  (|CallParentFunction OtherActor) ; This node is disabled and will not be called.\nDrag off pins to build functionality.
)

(event EventTick
  (params (DeltaSeconds :type Float%20%28single-precision%29))
  (|CallParentFunction DeltaSeconds) ; This node is disabled and will not be called.\nDrag off pins to build functionality.
)

(fn ConstructionScript
  (|CallParentFunction))

(fn PrimaryFire
  (params (location :type Vector :default "0, 0, 0") (rotation :type Rotator :default "0, 0, 0"))
  (bind _returnvalue (Utilities|Time|SetTimerbyFunctionName self "EndCooldown" (Variables|Default|GetWeaponCooldown)))
  (Variables|Default|SetCooldownTimerHadle _returnvalue)
  (return true))

(fn Attack
  (params (Location :type Vector) (Rotation :type Rotator))
  (bind (_outhit _returnvalue) (Collision|LineTraceByChannel Location (+ Location (* (Math|Vector|GetForwardVector Rotation) 200)) "TraceTypeQuery1" false 0 "ForDuration"))
  (if _returnvalue
    (Game|Damage|ApplyPointDamage (.HitActor (Collision|BreakHitResult _outhit)) (Variables|Default|GetPrimaryDamage) (.TraceStart (Collision|BreakHitResult _outhit)) _outhit 0 0 "/Script/Engine.DamageType")
    (Utilities|IsValid (.PhysMat (Collision|BreakHitResult _outhit))
      (:Is%20Valid
        (bind _returnvalue_2 (Utilities|GetDataTableRow "/Game/DataTable/DT_BulletHitEffects.DT_BulletHitEffects" (Utilities|String|StringToName (Utilities|String|EnumtoString (Variables|/Script/Engine.PhysicalMaterial|GetSurfaceType (.PhysMat (Collision|BreakHitResult _outhit))))))
          (:then
            (Effects|SpawnEmitteratLocation (.ParticleEffect (Utilities|Struct|BreakS_BulletHitEffect _returnvalue_2)) (.Location (Collision|BreakHitResult _outhit)) (Math|Rotator|FindLookatRotation Location (.Location (Collision|BreakHitResult _outhit))))
            (Audio|PlaySoundatLocation (.Sound (Utilities|Struct|BreakS_BulletHitEffect _returnvalue_2)) (.Location (Collision|BreakHitResult _outhit)) "0, 0, 0" 1.0 1.0 0.0 0 0 0)
            (bind _returnvalue_3 (Class|GameplayStatics|SpawnDecalAttached (Utilities|Array|Get(acopy) (.DecalMaterial (Utilities|Struct|BreakS_BulletHitEffect _returnvalue_2)) (Math|Random|RandomInteger (- (Utilities|Array|Length (.DecalMaterial (Utilities|Struct|BreakS_BulletHitEffect _returnvalue_2))) 1))) "2.000000,4.000000,4.000000" (.HitComponent (Collision|BreakHitResult _outhit)) "None" (.Location (Collision|BreakHitResult _outhit)) (Math|Rotator|FindLookatRotation Location (.Location (Collision|BreakHitResult _outhit))) "KeepWorldPosition" 0.0))
            (Rendering|Components|Decal|SetFadeScreenSize _returnvalue_3 0.001))
          (:RowNotFound
            (bind _returnvalue_4 (Utilities|GetDataTableRow "/Game/DataTable/DT_BulletHitEffects.DT_BulletHitEffects" "Default" :!label _label)
              (:then
                (Effects|SpawnEmitteratLocation (.ParticleEffect (Utilities|Struct|BreakS_BulletHitEffect _returnvalue_4)) (.Location (Collision|BreakHitResult _outhit)) (Math|Rotator|FindLookatRotation Location (.Location (Collision|BreakHitResult _outhit))))
                (Audio|PlaySoundatLocation (.Sound (Utilities|Struct|BreakS_BulletHitEffect _returnvalue_4)) (.Location (Collision|BreakHitResult _outhit)) "0, 0, 0" 1.0 1.0 0.0 0 0 0)
                (bind _returnvalue_5 (Class|GameplayStatics|SpawnDecalAttached (Utilities|Array|Get(acopy) (.DecalMaterial (Utilities|Struct|BreakS_BulletHitEffect _returnvalue_4)) (Math|Random|RandomInteger (- (Utilities|Array|Length (.DecalMaterial (Utilities|Struct|BreakS_BulletHitEffect _returnvalue_4))) 1))) "2.000000,4.000000,4.000000" (.HitComponent (Collision|BreakHitResult _outhit)) "None" (.Location (Collision|BreakHitResult _outhit)) (Math|Rotator|FindLookatRotation Location (.Location (Collision|BreakHitResult _outhit))) "KeepWorldPosition" 0.0))
                (Rendering|Components|Decal|SetFadeScreenSize _returnvalue_5 0.001))))))
      (:Is%20Not%20Valid
        (goto _label)))))