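; Save-system manager actor that keeps destroyed actors gone after a load, using a list of their names in Actors.
; On ActorLoaded, it scans every actor in the level and destroys any whose display name matches a list entry; nothing here fills that list.
; Disconnected graphs hold an unused tag-based alternative using NeedsAdditionalSaveInfo and Saved, and ComponentsToSave returns nothing.
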(event EventBeginPlay)

(event Collision|EventActorBeginOverlap
  (params (OtherActor :type Actor%20Object%20Reference)))

(event EventTick
  (params (DeltaSeconds :type Float%20%28single-precision%29)))

(event EventActorLoaded
  (bind _outactors (Actor|GetAllActorsOfClass "/Script/Engine.Actor"))
  (for _array_element _outactors
    (for _array_element_2 (Variables|Default|GetActors)
      (if (Utilities|Enum|Equal(Enum) _array_element_2 (Utilities|GetDisplayName _array_element))
        (Utilities|IsValid _array_element
          (:Is%20Valid
            (Actor|DestroyActor _array_element)))))))

(fn ConstructionScript)

(fn ComponentstoSave
  (return 0))