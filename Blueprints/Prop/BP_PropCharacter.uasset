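; Player character, apparently for a prop, that takes damage, interacts and carries physics objects.
; Fast looping timers replace Tick to zero mesh pitch, snap the mesh to traced ground unless jumping, move the physics-handle target, and destroy the actor at zero health.
; Camera traces drive interact messages and grab/release toggling.
; Two hard-coded keys reshape the capsule, counter-scaling the mesh.
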(event Custom|UpdateMeshRotation_Event
  (bind _capsulecomponent (Variables|Default|GetCapsuleComponent))
  (bind _playermesh (Variables|Default|GetPlayerMesh))
  (bind _returnvalue (Transformation|GetWorldLocation _capsulecomponent))
  (bind _returnvalue_2 (Transformation|GetWorldRotation _playermesh))
  (bind (_roll _pitch _yaw) (Math|Rotator|BreakRotator _returnvalue_2))
  (Transformation|SetWorldRotation _playermesh (Math|Rotator|MakeRotator _roll 0.0 _yaw) false false)
  (if (not (Variables|Default|GetbPressedJump))
    (bind (_outhit _returnvalue_3) (Collision|LineTraceByChannel _returnvalue (+ _returnvalue "0, 0,-100.000000") "TraceTypeQuery1" false 0 "None"))
    (if _returnvalue_3
      (Transformation|SetRelativeLocation (Variables|Default|GetPlayerMesh) (.Location (Math|Transform|BreakTransform (Math|Transform|MakeRelativeTransform (Math|Conversions|ToTransform(Vector) (.Location (Collision|BreakHitResult _outhit))) (Transformation|GetActorTransform)))) false false))
    (else
      (Transformation|SetRelativeLocation (Variables|Default|GetPlayerMesh) "0, 0, 0" false false))))

(event Custom|UdpatePhysHandle_Event
  (bind _camera (Variables|Default|GetCamera))
  (Physics|Components|PhysicsHandle|SetTargetLocation (Variables|Default|GetPhysicsHandle) (+ (Transformation|GetWorldLocation _camera) (* (Math|Vector|GetForwardVector _camera) 600))))

(event Custom|UpdateHealth_Event
  (if (<= (Variables|Default|GetHealth) 0.0)
    (Actor|DestroyActor)))

(event EventBeginPlay
  (Utilities|Time|SetTimerbyEvent (delegate Custom|UpdateMeshRotation_Event) 0.01 true)
  (Utilities|Time|SetTimerbyEvent (delegate Custom|UdpatePhysHandle_Event) 0.01 true)
  (Utilities|Time|SetTimerbyEvent (delegate Custom|UpdateHealth_Event) 0.01 true))

(event Collision|EventActorBeginOverlap
  (params (OtherActor :type Actor%20Object%20Reference)))

(event EventTick
  (params (DeltaSeconds :type Float%20%28single-precision%29)))

(event EventUse
  (bind _camera (Variables|Default|GetCamera))
  (bind _returnvalue (Transformation|GetWorldLocation _camera))
  (bind (_outhit _returnvalue_2) (Collision|LineTraceByChannel _returnvalue (+ _returnvalue (* (Math|Vector|GetForwardVector _camera) 600)) "TraceTypeQuery1" false (Utilities|Array|MakeArray self) "None"))
  (if _returnvalue_2
    (Class|InteractionInterface|Interact(Message) (.HitActor (Collision|BreakHitResult _outhit)) self (.HitComponent (Collision|BreakHitResult _outhit)))))

(event Game|Damage|EventAnyDamage
  (params (Damage :type Float%20%28single-precision%29) (DamageType :type Damage%20Type%20Object%20Reference) (InstigatedBy :type Controller%20Object%20Reference) (DamageCauser :type Actor%20Object%20Reference))
  (bind _output_get (Variables|Default|SetHealth (- (Variables|Default|GetHealth) Damage)))
  (Development|PrintString (Utilities|String|ToString(Float) _output_get)))

(event Input|ActionEvents|InputActionPickupObject
  (params (Key :type Key%20Structure :default "None"))
  (bind _camera (Variables|Default|GetCamera))
  (bind _physicshandle (Variables|Default|GetPhysicsHandle))
  (bind _returnvalue (Transformation|GetWorldLocation _camera))
  (:Pressed
    (Utilities|IsValid (Class|PhysicsHandleComponent|GetGrabbedComponent _physicshandle)
      (:Is%20Valid
        (Physics|Components|PhysicsHandle|ReleaseComponent _physicshandle))
      (:Is%20Not%20Valid
        (bind (_outhit _returnvalue_2) (Collision|LineTraceByChannel _returnvalue (+ _returnvalue (* (Math|Vector|GetForwardVector _camera) 600)) "TraceTypeQuery1" false (Utilities|Array|MakeArray self) "None"))
        (if _returnvalue_2
          (Physics|Components|PhysicsHandle|GrabComponentatLocationwithRotation _physicshandle (.HitComponent (Collision|BreakHitResult _outhit)) "None" (.Location (Collision|BreakHitResult _outhit)) "0, 0, 0"))))))

(event Input|KeyboardEvents|8
  (params (Key :type Key%20Structure :default "None"))
  (:Pressed
    (Transformation|SetWorldScale3D (Variables|Default|GetCapsuleComponent) "1.000000,1.000000,100.000000")
    (Transformation|SetRelativeScale3D (Variables|Default|GetPlayerMesh) "1.000000,1.000000,0.010000")))

(event Input|KeyboardEvents|9
  (params (Key :type Key%20Structure :default "None"))
  (:Pressed
    (Transformation|SetWorldScale3D (Variables|Default|GetCapsuleComponent) "2.000000,1.000000,0.100000")
    (Transformation|SetRelativeScale3D (Variables|Default|GetPlayerMesh) (Math|Vector|MakeVector 0.5 1.0 (/ 1.0 0.1)))))

(fn ConstructionScript)