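; Legacy physics prop that floats in water and, when interacted with, passes its mesh, health and capsule size to a PropCharacter for prop-hunt disguises.
; Construction toggles physics simulation, Tick applies buoyancy, and hard hits play an impact sound.
; Scrape audio depends on speed and IsTouchingAnything, whose return is disconnected, so the sound never starts.
; Health and key functions are stubs returning false.
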(event OnComponentHit(StaticMesh)
  (params (HitComponent :type Primitive%20Component%20Object%20Reference) (OtherActor :type Actor%20Object%20Reference) (OtherComp :type Primitive%20Component%20Object%20Reference) (NormalImpulse :type Vector :default "0, 0, 0") (Hit :type Hit%20Result%20Structure%20%28by%20ref%29))
  (if (> (Math|Vector|VectorLength NormalImpulse) (Variables|Default|GetMinImpulse))
    (Audio|PlaySoundatLocation (Variables|Default|GetOnHitSound) (.Location (Collision|BreakHitResult Hit)) "0, 0, 0" 1.0 1.0 0.0 "/Game/SuperGrid/TutorialLevel/SoundEffects/Attenuation_Ambient.Attenuation_Ambient" 0 0)))

(event OnComponentBeginOverlap(Box)
  (params (OverlappedComponent :type Primitive%20Component%20Object%20Reference) (OtherActor :type Actor%20Object%20Reference) (OtherComp :type Primitive%20Component%20Object%20Reference) (OtherBodyIndex :type Integer) (bFromSweep :type Boolean) (SweepResult :type Hit%20Result%20Structure%20%28by%20ref%29)))

(event EventBeginPlay
  (Collision|IgnoreActorwhenMoving (Variables|Default|GetBox) self true))

(event Collision|EventActorBeginOverlap
  (params (OtherActor :type Actor%20Object%20Reference)))

(event EventTick
  (params (DeltaSeconds :type Float%20%28single-precision%29))
  (bind _returnvalue (Transformation|GetVelocity))
  (bind _scrape_sound (Variables|Default|Getscrape_sound))
  (bind _returnvalue_2 (Math|Vector|VectorLength _returnvalue))
  (CallFunction|BuoyancyFunction (Variables|Default|GetStaticMesh) (Variables|Default|GetBouyancy) "ObjectTypeQuery8")
  (Development|PrintString (Utilities|String|ToString(Float) _returnvalue_2) false true "(R=0.000000,G=0.660000,B=1.000000,A=1.000000)" 0.01)
  (Development|PrintString (Utilities|String|ToString(Boolean) (CallFunction|IsTouchingAnything)) false true "(R=1.000000,G=0.093690,B=0.103637,A=1.000000)" 0.01)
  (if (CallFunction|IsTouchingAnything)
    (Utilities|IsValid _scrape_sound
      (:Is%20Valid
        (if (> _returnvalue_2 1e+01)
          (switch Utilities|FlowControl|Switch|SwitchonEAudioComponentPlayState (Audio|Components|Audio|GetPlayState _scrape_sound)
            (:Stopped
              (Audio|Components|Audio|Play _scrape_sound 0.0))
            (:Paused
              (Class|AudioComponent|SetPaused _scrape_sound false)))
          (else
            (Class|AudioComponent|SetPaused _scrape_sound true :!label _label)))))
    (else
      (goto _label))))

(event EventInteract
  (params (interactor :type Actor%20Object%20Reference) (interactedComponent :type Primitive%20Component%20Object%20Reference))
  (bind _propinfo (Variables|Default|GetPropInfo))
  (bind (_health _capsulehalfheight _caplusewidth _caplusescale) (Utilities|Struct|BreakS_PropInfo _propinfo))
  ;[1 1 1] from "prophunt" days
  (bind _asprop_character (Utilities|Casting|CastToPropCharacter interactor))
  (Class|PropCharacter|ChangeProp _asprop_character (Variables|/Script/Engine.StaticMeshComponent|GetStaticMesh (Variables|Default|GetStaticMesh)) _health _caplusewidth _capsulehalfheight _caplusescale))

(fn ConstructionScript
  (Physics|SetSimulatePhysics (Variables|Default|GetStaticMesh) (Variables|Default|GetHasPhysics?)))

(fn IsTouchingAnything
  (for _array_element (Collision|GetOverlappingActors (Variables|Default|GetBox) "/Script/Engine.Actor" :!class /Script/Engine.PrimitiveComponent)
    (Utilities|Casting|CastToWaterBody_BP0 _array_element)))

(fn AddHealth
  (params (amountOfHealth :type Float%20%28single-precision%29))
  (return false))

(fn HasKeywithId
  (params (id :type Integer))
  (return false))

(fn RemoveKey
  (params (KeyId :type Integer))
  (return false))