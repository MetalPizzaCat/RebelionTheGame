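; Physics prop that floats in water, reacts to collisions and gets pushed by grenade blasts.
; Tick runs the buoyancy function on the mesh, and mesh hits are forwarded to OnPropHit.
; Water impacts spawn a tinted splash emitter at the scrape sound's location.
; Radial damage applies a mesh impulse only from BP_GrenadeBase causers, along the damage trace and scaled by damage radius minus hit distance.
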(event OnComponentHit(Mesh)
  (params (HitComponent :type Primitive%20Component%20Object%20Reference) (OtherActor :type Actor%20Object%20Reference) (OtherComp :type Primitive%20Component%20Object%20Reference) (NormalImpulse :type Vector :default "0, 0, 0") (Hit :type Hit%20Result%20Structure%20%28by%20ref%29))
  (Class|PropBase|OnPropHit HitComponent OtherActor OtherComp NormalImpulse Hit))

(event EventBeginPlay)

(event Collision|EventActorBeginOverlap
  (params (OtherActor :type Actor%20Object%20Reference)))

(event EventTick
  (params (DeltaSeconds :type Float%20%28single-precision%29))
  (|CallParentFunction DeltaSeconds)
  (CallFunction|BuoyancyFunction (Variables|Character|GetMesh) (Variables|Default|GetBouyancy) "ObjectTypeQuery8"))

(event EventWaterImpact
  (bind _returnvalue (Effects|SpawnEmitteratLocation "/Game/_Marvelmaster_infinite_reactive_water_/Particles/Splash_PS.Splash_PS" (Transformation|GetWorldLocation (Variables|Default|GetScrapeSound))))
  (Effects|Components|ParticleSystem|SetColorParameter _returnvalue "color" "(R=0.817708,G=0.676797,B=0.185036,A=0.500000)"))

(event Game|Damage|EventRadialDamage
  (params (DamageReceived :type Float%20%28single-precision%29) (DamageType :type Damage%20Type%20Object%20Reference) (Origin :type Vector :default "0, 0, 0") (HitInfo :type Hit%20Result%20Structure%20%28by%20ref%29) (InstigatedBy :type Controller%20Object%20Reference) (DamageCauser :type Actor%20Object%20Reference))
  (bind (_impluse _hitlcoation) (HitVelocity|CalculateHitVelocity Origin HitInfo DamageCauser))
  (if (Physics|IsSimulatingPhysics (Variables|Character|GetMesh) "None")
    (Physics|AddImpulseatLocation (Variables|Character|GetMesh) _impluse _hitlcoation "None")))

(fn ConstructionScript)

(fn CalculateHitVelocity
  (params (HitFromDirection :type Vector) (HitInfo :type Hit%20Result%20Structure) (DamageCauser :type Actor%20Object%20Reference))
  (bind (_bblockinghit _binitialoverlap _time _distance _location _impactpoint _normal _impactnormal _physmat _hitactor _hitcomponent _hitbonename _hititem _faceindex _tracestart _traceend) (Collision|BreakHitResult HitInfo))
  (Utilities|IsValid DamageCauser
    (:Is%20Valid
      (bind _asbp_grenade_base (Utilities|Casting|CastToBP_GrenadeBase DamageCauser)
        (:then
          (return (* (- _traceend _tracestart) (* (- (Variables|/Game/Blueprints/Weapons/BP_GrenadeBase.BP_GrenadeBase_C|GetDamageRadius _asbp_grenade_base) _distance) 0.5)) _location))
        (:CastFailed
          _)))
    (:Is%20Not%20Valid
      _))
  (return "0, 0, 0" "0, 0, 0"))

(fn ComponentstoSave
  (return 0))