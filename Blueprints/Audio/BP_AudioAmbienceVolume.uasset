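; BP_AudioAmbienceVolume is a box volume that plays ambient audio when a PropHuntCharacter enters and stops it after a short delay on exit.
; Both overlap events set CurrenltySupposedToPlay to true, including the exit, and ActorLoaded reads that flag to restart or stop the audio.
; Construction applies DefaultVolume; a separate Stop function halts audio only if StopCompletly is set, with its lowered-volume path left unconnected.
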(event OnComponentBeginOverlap(Box)
  (params (OverlappedComponent :type Primitive%20Component%20Object%20Reference) (OtherActor :type Actor%20Object%20Reference) (OtherComp :type Primitive%20Component%20Object%20Reference) (OtherBodyIndex :type Integer) (bFromSweep :type Boolean) (SweepResult :type Hit%20Result%20Structure%20%28by%20ref%29))
  (Utilities|Casting|CastToPropHuntCharacter OtherActor)
  (Variables|Default|SetCurrenltySupposedToPlay true)
  (Audio|Components|Audio|Play (Variables|Default|GetAudio) 0.0))

(event OnComponentEndOverlap(Box)
  (params (OverlappedComponent :type Primitive%20Component%20Object%20Reference) (OtherActor :type Actor%20Object%20Reference) (OtherComp :type Primitive%20Component%20Object%20Reference) (OtherBodyIndex :type Integer))
  (Utilities|Casting|CastToPropHuntCharacter OtherActor)
  (Variables|Default|SetCurrenltySupposedToPlay true)
  (Audio|Components|Audio|StopDelayed (Variables|Default|GetAudio) 0.5))

(event EventBeginPlay)

(event Collision|EventActorBeginOverlap
  (params (OtherActor :type Actor%20Object%20Reference)))

(event EventTick
  (params (DeltaSeconds :type Float%20%28single-precision%29)))

(event EventActorLoaded
  (bind _audio (Variables|Default|GetAudio))
  (if (Variables|Default|GetCurrenltySupposedToPlay)
    (Audio|Components|Audio|Play _audio 0.0)
    (else
      (Audio|Components|Audio|StopDelayed _audio 0.0))))

(fn ConstructionScript
  (Variables|/Script/Engine.AudioComponent|SetVolumeMultiplier (Variables|Default|GetAudio) (Variables|Default|GetDefaultVolume)))

(fn Stop
  (if (Variables|Default|GetStopCompletly)
    (Audio|Components|Audio|Stop (Variables|Default|GetAudio))))

(fn ComponentstoSave
  (return 0))