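; BP_bed is a placeable bed building that validates its placement and becomes solid once construction finishes.
; CanBeBuilt passes only when the footprint Box and four walking-place boxes each overlap no more than one actor.
; Until Built, Tick repeats that check and shows the Cube as a blocked-placement indicator when it fails.
; OnBuildFinished enables query and physics collision on the mesh, blocking pawns, physics bodies and world objects.
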(event OnComponentBeginOverlap(Box)
  (params (OverlappedComponent :type Primitive%20Component%20Object%20Reference) (OtherActor :type Actor%20Object%20Reference) (OtherComp :type Primitive%20Component%20Object%20Reference) (OtherBodyIndex :type Integer) (bFromSweep :type Boolean) (SweepResult :type Hit%20Result%20Structure%20%28by%20ref%29)))

(event Custom|OnBuildStarted_1)

(event EventBeginPlay)

(event EventOnBuildFinished
  (bind _staticmesh (Variables|Default|GetStaticMesh))
  (Collision|SetCollisionEnabled _staticmesh "QueryAndPhysics")
  (Collision|SetCollisionResponsetoChannel _staticmesh "ECC_PhysicsBody" "ECR_Block")
  (Collision|SetCollisionResponsetoChannel _staticmesh "ECC_Pawn" "ECR_Block")
  (Collision|SetCollisionResponsetoChannel _staticmesh "ECC_WorldStatic" "ECR_Block")
  (Collision|SetCollisionResponsetoChannel _staticmesh "ECC_WorldDynamic" "ECR_Block"))

(event EventTick
  (params (DeltaSeconds :type Float%20%28single-precision%29))
  (if (not (Variables|Default|GetbBuilt))
    (Rendering|SetVisibility (Variables|Default|GetCube) (not (Math|Boolean|ANDBoolean (not (> (Utilities|Array|Length (Collision|GetOverlappingActors (Variables|Default|GetBox) "/Script/Engine.Actor" :!class /Script/Engine.PrimitiveComponent)) 1)) (not (> (Utilities|Array|Length (Collision|GetOverlappingActors (Variables|Default|GetBoxWalkingPlace) "/Script/Engine.Actor" :!class /Script/Engine.PrimitiveComponent)) 1)) (not (> (Utilities|Array|Length (Collision|GetOverlappingActors (Variables|Default|GetBoxWalkingPlace1) "/Script/Engine.Actor" :!class /Script/Engine.PrimitiveComponent)) 1)) (not (> (Utilities|Array|Length (Collision|GetOverlappingActors (Variables|Default|GetBoxWalkingPlace2) "/Script/Engine.Actor" :!class /Script/Engine.PrimitiveComponent)) 1)) (not (> (Utilities|Array|Length (Collision|GetOverlappingActors (Variables|Default|GetBoxWalkingPlace3) "/Script/Engine.Actor" :!class /Script/Engine.PrimitiveComponent)) 1)))) false)))

(fn ConstructionScript)

(fn CanbeBuilt
  (return (Math|Boolean|ANDBoolean (not (> (Utilities|Array|Length (Collision|GetOverlappingActors (Variables|Default|GetBox) "/Script/Engine.Actor" :!class /Script/Engine.PrimitiveComponent)) 1)) (not (> (Utilities|Array|Length (Collision|GetOverlappingActors (Variables|Default|GetBoxWalkingPlace) "/Script/Engine.Actor" :!class /Script/Engine.PrimitiveComponent)) 1)) (not (> (Utilities|Array|Length (Collision|GetOverlappingActors (Variables|Default|GetBoxWalkingPlace1) "/Script/Engine.Actor" :!class /Script/Engine.PrimitiveComponent)) 1)) (not (> (Utilities|Array|Length (Collision|GetOverlappingActors (Variables|Default|GetBoxWalkingPlace2) "/Script/Engine.Actor" :!class /Script/Engine.PrimitiveComponent)) 1)) (not (> (Utilities|Array|Length (Collision|GetOverlappingActors (Variables|Default|GetBoxWalkingPlace3) "/Script/Engine.Actor" :!class /Script/Engine.PrimitiveComponent)) 1)))))